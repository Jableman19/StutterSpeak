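; VR game mode that auto-pauses motion controllers and music when the app loses input focus or the headset comes off, in packaged builds only.
; Tick polls focus and HMD worn state, using a Pause flag so each transition fires once.
; Pausing hides each BP_MotionController, drops its held actor, sets it paused and fades music through MusicManager_Blueprint.
; Resuming unhides and unpauses the controllers, then calls menu music.
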(event `self.ReceiveTick`
  (params (DeltaSeconds :type "Float (single-precision)"))
  (if (`KismetSystemLibrary.IsPackagedForDistribution`)
    (if (`OculusFunctionLibrary.HasInputFocus`)
      (if (`|EnumEquality` (`HeadMountedDisplayFunctionLibrary.GetHMDWornState`) "Worn")
        (if (`self.Pause`)
          (bind _outactors (`GameplayStatics.GetAllActorsOfClass` "/Game/Starter_Content/VirtualRealityBP/Blueprints/BP_MotionController.BP_MotionController_C"))
          (for _array_element _outactors
            (bind _asbp_motion_controller (cast `/Game/Starter_Content/VirtualRealityBP/Blueprints/BP_MotionController` _array_element))
            (`self.SetActorHiddenInGame` _array_element false)
            (`self.SetActorHiddenInGame` _asbp_motion_controller false)
            (set `/Game/Starter_Content/VirtualRealityBP/Blueprints/BP_MotionController.Paused` false _array_element)
            (set `Actor.bGenerateOverlapEventsDuringLevelStreaming` true _array_element))
          (bind _outactors_2 (`GameplayStatics.GetAllActorsOfClass` "/Game/Stutter_Speak_Content/Managers/MusicManager_Blueprint.MusicManager_Blueprint_C"))
          (bind _asmusic_manager_blueprint (cast `/Game/Stutter_Speak_Content/Managers/MusicManager_Blueprint` (`|GetArrayItem` _outactors_2)))
          (`/Game/Stutter_Speak_Content/Managers/MusicManager_Blueprint.MenuMusicCall` _asmusic_manager_blueprint)
          (set `self.Pause` false))
        (else
          (if (not (`self.Pause`)) :!label _label
            (bind _outactors_3 (`GameplayStatics.GetAllActorsOfClass` "/Game/Starter_Content/VirtualRealityBP/Blueprints/BP_MotionController.BP_MotionController_C"))
            (for _array_element_2 _outactors_3
              (bind _asbp_motion_controller_2 (cast `/Game/Starter_Content/VirtualRealityBP/Blueprints/BP_MotionController` _array_element_2))
              (`self.SetActorHiddenInGame` _array_element_2 true)
              (`self.SetActorHiddenInGame` _asbp_motion_controller_2 true)
              (`/Game/Starter_Content/VirtualRealityBP/Blueprints/BP_MotionController.DropActor` _asbp_motion_controller_2)
              (set `/Game/Starter_Content/VirtualRealityBP/Blueprints/BP_MotionController.Paused` true _array_element_2)
              (set `Actor.bGenerateOverlapEventsDuringLevelStreaming` false _array_element_2))
            (bind _outactors_4 (`GameplayStatics.GetAllActorsOfClass` "/Game/Stutter_Speak_Content/Managers/MusicManager_Blueprint.MusicManager_Blueprint_C"))
            (bind _asmusic_manager_blueprint_2 (cast `/Game/Stutter_Speak_Content/Managers/MusicManager_Blueprint` (`|GetArrayItem` _outactors_4)))
            (`/Game/Stutter_Speak_Content/Managers/MusicManager_Blueprint.MusicFade` _asmusic_manager_blueprint_2)
            (set `self.Pause` true))))
      (else
        (goto _label)))))

(event `self.ReceiveBeginPlay`)

(fn `UserConstructionScript`)