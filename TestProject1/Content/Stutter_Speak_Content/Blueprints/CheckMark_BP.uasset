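; CheckMark_BP is a pressable confirm button, hidden at start, that a hand pushes to load a speech from the menu.
; ConfirmByBegin reveals and raises the mesh with query collision, while ConfirmByCancel lowers and hides it.
; An overlap by a HandHit component from above sinks the armed button, plays a lower-pitched sound and calls SpeechLoaderByDetailsPanel on the level's MenuWorldLevelHolder.
; Each press then disarms the button until a confirm event re-arms it.
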(event `ConfirmByCancel`
  (bind (_returnvalue_location _returnvalue_rotation) (`KismetMathLibrary.BreakTransform` (`SceneComponent.GetRelativeTransform` (`self.StaticMeshComponent`))))
  (`KismetSystemLibrary.MoveComponentTo` (`self.StaticMeshComponent`) (`self.DownLocation`) _returnvalue_rotation false false 1.0)
  (set `self.ButtonOn` true)
  (`self.SetActorHiddenInGame` true)
  (`PrimitiveComponent.SetCollisionEnabled` (`self.StaticMeshComponent`) "NoCollision"))

(event `ConfirmByBegin`
  (bind (_returnvalue_location _returnvalue_rotation) (`KismetMathLibrary.BreakTransform` (`SceneComponent.GetRelativeTransform` (`self.StaticMeshComponent`))))
  (`KismetSystemLibrary.MoveComponentTo` (`self.StaticMeshComponent`) (`self.UpLocation`) _returnvalue_rotation false false 1.0)
  (set `self.ButtonOn` true)
  (`self.SetActorHiddenInGame` false)
  (`PrimitiveComponent.SetCollisionEnabled` (`self.StaticMeshComponent`) "QueryOnly"))

(event `self.ReceiveBeginPlay`
  (bind _returnvalue (`SceneComponent.GetRelativeTransform` (`self.StaticMeshComponent`)))
  (bind (_returnvalue_location _returnvalue_rotation _returnvalue_scale) (`KismetMathLibrary.BreakTransform` (`SceneComponent.GetRelativeTransform` (`self.StaticMeshComponent`))))
  (`self.SetActorHiddenInGame` true)
  (`PrimitiveComponent.SetCollisionEnabled` (`self.StaticMeshComponent`) "NoCollision")
  (`KismetSystemLibrary.Delay` 1.0)
  (set `self.UpLocation` (`KismetMathLibrary.MakeVector` (.x (.location _returnvalue)) (.y (.location _returnvalue)) (.z (.location _returnvalue))))
  (bind _output_get (set `self.DownLocation` (`KismetMathLibrary.MakeVector` (.x (.location _returnvalue)) (.y (.location _returnvalue)) (- (.z (.location _returnvalue)) 30.0))))
  (`SceneComponent.K2_SetRelativeTransform` (`self.StaticMeshComponent`) (`KismetMathLibrary.MakeTransform` _output_get _returnvalue_rotation _returnvalue_scale) false false))

(event `self.StaticMeshComponent.OnComponentBeginOverlap`
  (params (OverlappedComponent :type "PrimitiveComponent Object Reference") (OtherActor :type "Actor Object Reference") (OtherComp :type "PrimitiveComponent Object Reference") (OtherBodyIndex :type Integer) (bFromSweep :type Boolean) (SweepResult :type "HitResult Structure (by ref)"))
  (bind (_returnvalue_x _returnvalue_y _returnvalue_z) (`KismetMathLibrary.BreakVector` (`SceneComponent.K2_GetComponentLocation` OtherComp)))
  (bind _sound (`self.Sound`))
  (bind (_returnvalue_x_2 _returnvalue_y_2 _returnvalue_z_2) (`KismetMathLibrary.BreakVector` (`SceneComponent.K2_GetComponentLocation` (`self.StaticMeshComponent`))))
  (bind (_returnvalue_location _returnvalue_rotation) (`KismetMathLibrary.BreakTransform` (`SceneComponent.GetRelativeTransform` (`self.StaticMeshComponent`))))
  ;[1 1 1] Pressed Down
  (if (`self.ButtonOn`)
    (if (> _returnvalue_z _returnvalue_z_2)
      (if (`KismetStringLibrary.EqualEqual_StrStr` (`KismetSystemLibrary.GetObjectName` OtherComp) "HandHit")
        (if (not (`self.isPressedDown`))
          (`KismetSystemLibrary.MoveComponentTo` (`self.StaticMeshComponent`) (`self.DownLocation`) _returnvalue_rotation false false 1.0)
          (`AudioComponent.SetPitchMultiplier` _sound 0.75)
          (`AudioComponent.Play` _sound 0.0)
          (set `self.isPressedDown` true)
          (bind _outactors (`GameplayStatics.GetAllActorsOfClass` "/Game/Stutter_Speak_Content/Managers/MenuWorldLevelHolder.MenuWorldLevelHolder_C"))
          (bind _asmenu_world_level_holder (cast `/Game/Stutter_Speak_Content/Managers/MenuWorldLevelHolder` (`|GetArrayItem` _outactors)))
          (`/Game/Stutter_Speak_Content/Managers/MenuWorldLevelHolder.SpeechLoaderByDetailsPanel` _asmenu_world_level_holder)
          (set `self.ButtonOn` false)
          (`KismetSystemLibrary.Delay` 0.35)
          (set `self.isPressedDown` false))))))

(fn `UserConstructionScript`)