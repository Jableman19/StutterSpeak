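; A hanging projector screen actor that displays rating, instruction and results UI on its Widget component in a speech-practice scene.
; On BeginPlay it creates and stores the fluency rater, results data and two retracking widgets, keeps the component's original widget as the effectiveness rater, then hides itself in game.
; Four custom events swap the created widgets onto the component; none of them unhides the screen or restores the effectiveness rater.
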(event `self.ReceiveBeginPlay`
  (bind _returnvalue (`|CreateWidget` "/Game/Stutter_Speak_Content/Widgets/Speech_World/FluencyRaterBP1.FluencyRaterBP1_C"))
  (set `self.Fluency Rater` _returnvalue)
  (bind _returnvalue_2 (`|CreateWidget` "/Game/Stutter_Speak_Content/Widgets/Speech_World/ResultsDataBP.ResultsDataBP_C"))
  (set `self.Results Data` _returnvalue_2)
  (bind _returnvalue_3 (`|CreateWidget` "/Game/Stutter_Speak_Content/Widgets/Speech_World/Retracking_Instructions.Retracking_Instructions_C"))
  (set `self.Retracking Instructions` _returnvalue_3)
  (bind _returnvalue_4 (`|CreateWidget` "/Game/Stutter_Speak_Content/Widgets/Speech_World/Retracking_Results.Retracking_Results_C"))
  (set `self.Retracking Results` _returnvalue_4)
  (set `self.Effectiveness Rater` (`WidgetComponent.GetWidget` (`self.Widget`)))
  (`self.SetActorHiddenInGame` true))

(event `ChangeWidget`
  (`WidgetComponent.SetWidget` (`self.Widget`) (`self.Fluency Rater`)))

(event `DisplayResults`
  (`WidgetComponent.SetWidget` (`self.Widget`) (`self.Results Data`)))

(event `DisplayInstructions`
  (`WidgetComponent.SetWidget` (`self.Widget`) (`self.Retracking Instructions`)))

(event `DisplayRetrackingResults`
  (`WidgetComponent.SetWidget` (`self.Widget`) (`self.Retracking Results`)))

(fn `UserConstructionScript`)