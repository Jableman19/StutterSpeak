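; SettingsBox is the in-game settings panel for text size, menu music, applause, stutter button and microphone color, driven by switch events.
; BeginPlay copies the saved values from the MenuGI game instance.
; Text size switches act as radio buttons, resetting the other two tagged SwitchBP actors' rotation and grabbability.
; Each change writes to MenuGI and saves through a shared call; the music toggle also notifies MusicManager_Blueprint.
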(event `self.ReceiveBeginPlay`
  ;[1 1 1] Checks Settings when created
  (bind _asmenu_gi (cast `/Game/Stutter_Speak_Content/Blueprints/MenuGI` (`GameplayStatics.GetGameInstance`)))
  (set `self.MicrophoneColor` (`/Game/Stutter_Speak_Content/Blueprints/MenuGI.MicrophoneColor` _asmenu_gi))
  (set `self.StutterButton` (`/Game/Stutter_Speak_Content/Blueprints/MenuGI.StutterButtonOn` _asmenu_gi))
  (set `self.Applause` (`/Game/Stutter_Speak_Content/Blueprints/MenuGI.Applause` _asmenu_gi))
  (set `self.Ambience` (`/Game/Stutter_Speak_Content/Blueprints/MenuGI.Ambience` _asmenu_gi))
  (set `self.MusicOn` (`/Game/Stutter_Speak_Content/Blueprints/MenuGI.MenuMusic` _asmenu_gi))
  (bind _textsize (`/Game/Stutter_Speak_Content/Blueprints/MenuGI.TextSize` _asmenu_gi))
  (if (`KismetStringLibrary.EqualEqual_StrStr` _textsize "Small")
    (set `self.LargeText` false)
    (set `self.MedText` false)
    (set `self.SmallText` true)
    (elif (`KismetStringLibrary.EqualEqual_StrStr` _textsize "Medium")
      (set `self.LargeText` false)
      (set `self.MedText` true)
      (set `self.SmallText` false)
      (else
        (set `self.LargeText` true)
        (set `self.MedText` false)
        (set `self.SmallText` false)))))

(event `LargeByLargeSwitch`
  (bind _outactors (`GameplayStatics.GetAllActorsOfClassWithTag` "/Game/Stutter_Speak_Content/Blueprints/SwitchBP.SwitchBP_C" "Small"))
  (bind _asswitch_bp (cast `/Game/Stutter_Speak_Content/Blueprints/SwitchBP` (`|GetArrayItem` _outactors)))
  (`SceneComponent.K2_SetRelativeRotation` (`/Game/Stutter_Speak_Content/Blueprints/SwitchBP.Switch` _asswitch_bp) (struct :`Roll` 30.0) false false)
  (set `/Game/Stutter_Speak_Content/Blueprints/SwitchBP.Grabbable` true _asswitch_bp)
  (bind _outactors_2 (`GameplayStatics.GetAllActorsOfClassWithTag` "/Game/Stutter_Speak_Content/Blueprints/SwitchBP.SwitchBP_C" "Medium"))
  (bind _asswitch_bp_2 (cast `/Game/Stutter_Speak_Content/Blueprints/SwitchBP` (`|GetArrayItem` _outactors_2)))
  (`SceneComponent.K2_SetRelativeRotation` (`/Game/Stutter_Speak_Content/Blueprints/SwitchBP.Switch` _asswitch_bp_2) (struct :`Roll` 30.0) false false)
  (set `/Game/Stutter_Speak_Content/Blueprints/SwitchBP.Grabbable` true _asswitch_bp_2)
  (set `self.LargeText` true)
  (set `self.MedText` false)
  (set `self.SmallText` false)
  (bind _asmenu_gi (cast `/Game/Stutter_Speak_Content/Blueprints/MenuGI` (`GameplayStatics.GetGameInstance`)))
  (set `/Game/Stutter_Speak_Content/Blueprints/MenuGI.TextSize` "Large" _asmenu_gi)
  ;[1 1 1] Saves Settins [Do on switch]
  (bind _asmenu_gi_2 (cast `/Game/Stutter_Speak_Content/Blueprints/MenuGI` (`GameplayStatics.GetGameInstance`) :!label _label))
  (`/Game/Stutter_Speak_Content/Blueprints/MenuGI.SavingSettingsDataBySettingsMenu` _asmenu_gi_2))

(event `MediumByMediumSwitch`
  (bind _outactors (`GameplayStatics.GetAllActorsOfClassWithTag` "/Game/Stutter_Speak_Content/Blueprints/SwitchBP.SwitchBP_C" "Small"))
  (bind _asswitch_bp (cast `/Game/Stutter_Speak_Content/Blueprints/SwitchBP` (`|GetArrayItem` _outactors)))
  (`SceneComponent.K2_SetRelativeRotation` (`/Game/Stutter_Speak_Content/Blueprints/SwitchBP.Switch` _asswitch_bp) (struct :`Roll` 30.0) false false)
  (set `/Game/Stutter_Speak_Content/Blueprints/SwitchBP.Grabbable` true _asswitch_bp)
  (bind _outactors_2 (`GameplayStatics.GetAllActorsOfClassWithTag` "/Game/Stutter_Speak_Content/Blueprints/SwitchBP.SwitchBP_C" "Large"))
  (bind _asswitch_bp_2 (cast `/Game/Stutter_Speak_Content/Blueprints/SwitchBP` (`|GetArrayItem` _outactors_2)))
  (`SceneComponent.K2_SetRelativeRotation` (`/Game/Stutter_Speak_Content/Blueprints/SwitchBP.Switch` _asswitch_bp_2) (struct :`Roll` 30.0) false false)
  (set `/Game/Stutter_Speak_Content/Blueprints/SwitchBP.Grabbable` true _asswitch_bp_2)
  (set `self.LargeText` false)
  (set `self.MedText` true)
  (set `self.SmallText` false)
  (bind _asmenu_gi (cast `/Game/Stutter_Speak_Content/Blueprints/MenuGI` (`GameplayStatics.GetGameInstance`)))
  (set `/Game/Stutter_Speak_Content/Blueprints/MenuGI.TextSize` "Medium" _asmenu_gi)
  (goto _label))

(event `SmallBySmallSwitch`
  (bind _outactors (`GameplayStatics.GetAllActorsOfClassWithTag` "/Game/Stutter_Speak_Content/Blueprints/SwitchBP.SwitchBP_C" "Large"))
  (bind _asswitch_bp (cast `/Game/Stutter_Speak_Content/Blueprints/SwitchBP` (`|GetArrayItem` _outactors)))
  (`SceneComponent.K2_SetRelativeRotation` (`/Game/Stutter_Speak_Content/Blueprints/SwitchBP.Switch` _asswitch_bp) (struct :`Roll` 30.0) false false)
  (set `/Game/Stutter_Speak_Content/Blueprints/SwitchBP.Grabbable` true _asswitch_bp)
  (bind _outactors_2 (`GameplayStatics.GetAllActorsOfClassWithTag` "/Game/Stutter_Speak_Content/Blueprints/SwitchBP.SwitchBP_C" "Medium"))
  (bind _asswitch_bp_2 (cast `/Game/Stutter_Speak_Content/Blueprints/SwitchBP` (`|GetArrayItem` _outactors_2)))
  (`SceneComponent.K2_SetRelativeRotation` (`/Game/Stutter_Speak_Content/Blueprints/SwitchBP.Switch` _asswitch_bp_2) (struct :`Roll` 30.0) false false)
  (set `/Game/Stutter_Speak_Content/Blueprints/SwitchBP.Grabbable` true _asswitch_bp_2)
  (set `self.LargeText` false)
  (set `self.MedText` false)
  (set `self.SmallText` true)
  (bind _asmenu_gi (cast `/Game/Stutter_Speak_Content/Blueprints/MenuGI` (`GameplayStatics.GetGameInstance`)))
  (set `/Game/Stutter_Speak_Content/Blueprints/MenuGI.TextSize` "Small" _asmenu_gi)
  (goto _label))

(event `MusicOnByMusicSwitch`
  (bind _asmenu_gi (cast `/Game/Stutter_Speak_Content/Blueprints/MenuGI` (`GameplayStatics.GetGameInstance`)))
  (bind _output_get (set `/Game/Stutter_Speak_Content/Blueprints/MenuGI.MenuMusic` (not (`self.MusicOn`)) _asmenu_gi))
  (set `self.MusicOn` _output_get)
  (bind _outactors (`GameplayStatics.GetAllActorsOfClass` "/Game/Stutter_Speak_Content/Managers/MusicManager_Blueprint.MusicManager_Blueprint_C"))
  (bind _asmusic_manager_blueprint (cast `/Game/Stutter_Speak_Content/Managers/MusicManager_Blueprint` (`|GetArrayItem` _outactors)))
  (`/Game/Stutter_Speak_Content/Managers/MusicManager_Blueprint.MenuMusicCall` _asmusic_manager_blueprint)
  (goto _label))

(event `ApplauseByApplauseSwitch`
  (bind _returnvalue (not (`self.Applause`)))
  (bind _asmenu_gi (cast `/Game/Stutter_Speak_Content/Blueprints/MenuGI` (`GameplayStatics.GetGameInstance`)))
  (set `/Game/Stutter_Speak_Content/Blueprints/MenuGI.Applause` _returnvalue _asmenu_gi)
  (set `self.Applause` _returnvalue)
  (goto _label))

(event `StutterButtonByStutterSwitch`
  (bind _returnvalue (not (`self.StutterButton`)))
  (bind _asmenu_gi (cast `/Game/Stutter_Speak_Content/Blueprints/MenuGI` (`GameplayStatics.GetGameInstance`)))
  (set `/Game/Stutter_Speak_Content/Blueprints/MenuGI.StutterButtonOn` _returnvalue _asmenu_gi)
  (set `self.StutterButton` _returnvalue)
  (goto _label))

(event `MicrophoneColorByMicSwitch`
  (bind _returnvalue (not (`self.MicrophoneColor`)))
  (bind _asmenu_gi (cast `/Game/Stutter_Speak_Content/Blueprints/MenuGI` (`GameplayStatics.GetGameInstance`)))
  (set `/Game/Stutter_Speak_Content/Blueprints/MenuGI.MicrophoneColor` _returnvalue _asmenu_gi)
  (set `self.MicrophoneColor` _returnvalue)
  (goto _label))

(fn `UserConstructionScript`)