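; VR projector that loads a grabbed floppy and shows its speech details or the credits on the projector screen.
; An active floppy entering GrabBox resets the previous one to spawn, leaves the hand, snaps to a hologram floppy's transform and slides in on a timeline.
; Screen and light-cone fades frame the swap, then the speech name is stored or the credits widget shown, and buttons update to match.
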(event `FadeInOnReset`
  (bind _outactors (`GameplayStatics.GetAllActorsOfClass` "/Game/Stutter_Speak_Content/Blueprints/ProjectorScreen_Blueprint.ProjectorScreen_Blueprint_C"))
  (bind _asprojector_screen_blueprint (cast `/Game/Stutter_Speak_Content/Blueprints/ProjectorScreen_Blueprint` (`|GetArrayItem` _outactors)))
  (if (not (`self.Beginning`))
    (`/Game/Stutter_Speak_Content/Blueprints/ProjectorScreen_Blueprint.ProjectorFadeIn` _asprojector_screen_blueprint)
    (bind _outactors_2 (`GameplayStatics.GetAllActorsOfClass` "/Game/Stutter_Speak_Content/Pre-Fabs/CompleteModels/Projection/projectorcone_Blueprint.projectorcone_Blueprint_C"))
    (bind _asprojectorcone_blueprint (cast `/Game/Stutter_Speak_Content/Pre-Fabs/CompleteModels/Projection/projectorcone_Blueprint` (`|GetArrayItem` _outactors_2)))
    (`/Game/Stutter_Speak_Content/Pre-Fabs/CompleteModels/Projection/projectorcone_Blueprint.Fade Out` _asprojectorcone_blueprint)
    (`KismetSystemLibrary.Delay` 1.0))
  (bind _asfloppy_text (cast `/Game/Stutter_Speak_Content/Widgets/Floppy_Text` (`WidgetComponent.GetWidget` (`/Game/Stutter_Speak_Content/Blueprints/Floppy.Floppy Name` (`self.Chosen Floppy`)))))
  (set `/Game/Stutter_Speak_Content/Widgets/Floppy_Text.Reset` true _asfloppy_text)
  (`/Game/Stutter_Speak_Content/Widgets/Floppy_Text.StoreSpeechNameByProjector` _asfloppy_text)
  (set `/Game/Stutter_Speak_Content/Widgets/Floppy_Text.Reset` false _asfloppy_text)
  (`/Game/Stutter_Speak_Content/Blueprints/ProjectorScreen_Blueprint.RevertByCancel` _asprojector_screen_blueprint)
  (`KismetSystemLibrary.Delay` 0.5)
  (bind _outactors_3 (`GameplayStatics.GetAllActorsOfClass` "/Game/Stutter_Speak_Content/Pre-Fabs/CompleteModels/Projection/projectorcone_Blueprint.projectorcone_Blueprint_C"))
  (bind _asprojectorcone_blueprint_2 (cast `/Game/Stutter_Speak_Content/Pre-Fabs/CompleteModels/Projection/projectorcone_Blueprint` (`|GetArrayItem` _outactors_3)))
  (`/Game/Stutter_Speak_Content/Pre-Fabs/CompleteModels/Projection/projectorcone_Blueprint.Fade in` _asprojectorcone_blueprint_2))

(event `self.ReceiveBeginPlay`
  (bind _outactors (`GameplayStatics.GetAllActorsOfClassWithTag` "/Script/Engine.SpotLight" "Projector")))

(event `self.GrabBox.OnComponentBeginOverlap`
  (params (OverlappedComponent :type "PrimitiveComponent Object Reference") (OtherActor :type "Actor Object Reference") (OtherComp :type "PrimitiveComponent Object Reference") (OtherBodyIndex :type Integer) (bFromSweep :type Boolean) (SweepResult :type "HitResult Structure (by ref)"))
  (bind _other_actor (`self.Other Actor`))
  (bind _chosen_floppy (`self.Chosen Floppy`))
  (bind _staticmesh (`/Game/Stutter_Speak_Content/Blueprints/Floppy.StaticMesh` _chosen_floppy))
  (bind _tags (`Actor.Tags` (`self.Other Actor`)))
  ;[0 0 0] Variables for later use
  (set `self.Overlapped Component` OverlappedComponent)
  (set `self.Other Actor` OtherActor)
  (set `self.Other Comp` OtherComp)
  ;[1 1 1] Checks if overlapping actor is a floppy
  (if (== (`|GetArrayItem` _tags) "floppy")
    (if (== (`|GetArrayItem` _tags (`KismetArrayLibrary.Array_LastIndex` _tags)) "Active")
      ;[1 1 1] Disables grab box collison during animation
      (`PrimitiveComponent.SetCollisionEnabled` (`self.Overlapped Component`) "NoCollision")
      (bind _outactors (`GameplayStatics.GetAllActorsOfClass` "/Game/Stutter_Speak_Content/Pre-Fabs/CompleteModels/BeginButton.BeginButton_C"))
      (bind _asbegin_button (cast `/Game/Stutter_Speak_Content/Pre-Fabs/CompleteModels/BeginButton` (`|GetArrayItem` _outactors)))
      (set `/Game/Stutter_Speak_Content/Pre-Fabs/CompleteModels/BeginButton.ButtonOn` false _asbegin_button)
      ;[1 1 1] Resetting current floppy
      (if (`self.Not First Time`)
        (bind _outactors_2 (`GameplayStatics.GetAllActorsOfClassWithTag` "/Game/Stutter_Speak_Content/Blueprints/Floppy.Floppy_C" (`|GetArrayItem` (`Actor.Tags` (`self.Current Floppy`)) 1)))
        (bind _asfloppy (cast `/Game/Stutter_Speak_Content/Blueprints/Floppy` (`|GetArrayItem` _outactors_2)))
        (`KismetSystemLibrary.Delay` 0.01)
        (`self.K2_SetActorLocationAndRotation` _asfloppy (`/Game/Stutter_Speak_Content/Blueprints/Floppy.Spawn Location` _asfloppy) (`/Game/Stutter_Speak_Content/Blueprints/Floppy.Spawn Rotation` _asfloppy) false false)
        (set `/Game/Stutter_Speak_Content/Blueprints/Floppy.Grabbable` true _asfloppy)
        (`|ExecutionSequence`
          (:`then_0`
            (bind _outactors_3 (`GameplayStatics.GetAllActorsOfClass` "/Game/Stutter_Speak_Content/Blueprints/Reset_Data_Base2_Blueprint.Reset_Data_Base2_Blueprint_C"))
            (bind _asreset_data_base_2_blueprint (cast `/Game/Stutter_Speak_Content/Blueprints/Reset_Data_Base2_Blueprint` (`|GetArrayItem` _outactors_3)))
            (bind _asreset_button_display (cast `/Game/Stutter_Speak_Content/Widgets/Menu_World_Widgets/Reset_Button_Display` (`WidgetComponent.GetWidget` (`/Game/Stutter_Speak_Content/Blueprints/Reset_Data_Base2_Blueprint.Widget` _asreset_data_base_2_blueprint))))
            (`/Game/Stutter_Speak_Content/Widgets/Menu_World_Widgets/Reset_Button_Display.StopDisplayingByProjector` _asreset_button_display)
            ;[1 1 1] Removes the floppy from the hand
            (bind _outactors_4 (`GameplayStatics.GetAllActorsOfClass` "/Game/Starter_Content/VirtualRealityBP/Blueprints/MotionControllerPawn.MotionControllerPawn_C" :!label _label))
            (bind _asmotion_controller_pawn (cast `/Game/Starter_Content/VirtualRealityBP/Blueprints/MotionControllerPawn` (`|GetArrayItem` _outactors_4)))
            ;[1 1 1] Checks which hand to remove the floppy from
            (bind _outactors_5 (`GameplayStatics.GetAllActorsOfClass` "/Game/Starter_Content/VirtualRealityBP/Blueprints/BP_MotionController.BP_MotionController_C"))
            (bind _asbp_motion_controller (cast `/Game/Starter_Content/VirtualRealityBP/Blueprints/BP_MotionController` (`|GetArrayItem` _outactors_5)))
            (bind _asbp_motion_controller_2 (cast `/Game/Starter_Content/VirtualRealityBP/Blueprints/BP_MotionController` (`|GetArrayItem` _outactors_5 1)))
            (if (== (`/Game/Starter_Content/VirtualRealityBP/Blueprints/BP_MotionController.AttachedActor` _asbp_motion_controller_2) _other_actor)
              (`/Game/Starter_Content/VirtualRealityBP/Blueprints/MotionControllerPawn.ReleaseByProjector(Right)` _asmotion_controller_pawn)
              (elif (== _other_actor (`/Game/Starter_Content/VirtualRealityBP/Blueprints/BP_MotionController.AttachedActor` _asbp_motion_controller))
                (`/Game/Starter_Content/VirtualRealityBP/Blueprints/MotionControllerPawn.ReleaseByProjector(Left)` _asmotion_controller_pawn)))
            ;[1 1 1] Turns off physics on the floppy for the animation
            (bind _outactors_6 (`GameplayStatics.GetAllActorsOfClassWithTag` "/Game/Stutter_Speak_Content/Blueprints/Floppy.Floppy_C" (`|GetArrayItem` (`Actor.Tags` (`self.Other Actor`)) 1)))
            (bind _output_get (set `self.Chosen Floppy` (`|GetArrayItem` _outactors_6)))
            (set `/Game/Stutter_Speak_Content/Blueprints/Floppy.Grabbable` false _output_get)
            (bind _staticmesh_2 (`/Game/Stutter_Speak_Content/Blueprints/Floppy.StaticMesh` _output_get))
            (`PrimitiveComponent.SetSimulatePhysics` _staticmesh_2 false)
            (`PrimitiveComponent.SetCollisionEnabled` _staticmesh_2 "NoCollision")
            (bind _outactors_7 (`GameplayStatics.GetAllActorsOfClassWithTag` "/Game/Stutter_Speak_Content/Blueprints/Floppy.Floppy_C" "Hologram"))
            (bind _asfloppy_2 (cast `/Game/Stutter_Speak_Content/Blueprints/Floppy` (`|GetArrayItem` _outactors_7)))
            (bind (_returnvalue_location _returnvalue_rotation) (`KismetMathLibrary.BreakTransform` (`self.GetTransform` _asfloppy_2)))
            ;[1 1 1] Grabs floppy from hand and runs animation of sliding into projector
            (`self.K2_SetActorLocationAndRotation` (`self.Other Actor`) _returnvalue_location _returnvalue_rotation false false)
            (bind _outactors_8 (`GameplayStatics.GetAllActorsOfClass` "/Game/Stutter_Speak_Content/Blueprints/ProjectorScreen_Blueprint.ProjectorScreen_Blueprint_C"))
            (bind _asprojector_screen_blueprint (cast `/Game/Stutter_Speak_Content/Blueprints/ProjectorScreen_Blueprint` (`|GetArrayItem` _outactors_8)))
            (`/Game/Stutter_Speak_Content/Blueprints/ProjectorScreen_Blueprint.ProjectorFadeIn` _asprojector_screen_blueprint)
            (if (not (`self.FirstFloppy`))
              ;[1 1 1] Light Turns Off and On
              (bind _outactors_9 (`GameplayStatics.GetAllActorsOfClass` "/Game/Stutter_Speak_Content/Pre-Fabs/CompleteModels/Projection/projectorcone_Blueprint.projectorcone_Blueprint_C"))
              (bind _asprojectorcone_blueprint (cast `/Game/Stutter_Speak_Content/Pre-Fabs/CompleteModels/Projection/projectorcone_Blueprint` (`|GetArrayItem` _outactors_9)))
              (`/Game/Stutter_Speak_Content/Pre-Fabs/CompleteModels/Projection/projectorcone_Blueprint.Fade Out` _asprojectorcone_blueprint))
            (bind _output_get_2 (set `self.NewVar_0` (`self.GetActorUpVector` _chosen_floppy)))
            (bind _output_get_3 (set `self.NewVar_1` (`SceneComponent.K2_GetComponentLocation` _staticmesh)))
            (bind (_direction _newtrack_0) (`Timeline|FloppyMove` :!via `PlayFromStart`)
              (:`Update`
                ;;[0 0 0] Always move the static mesh of the floppy
                (`SceneComponent.K2_SetWorldLocation` _staticmesh (+ (* _output_get_2 (* _newtrack_0 11.0)) _output_get_3) false false))
              (:`Finished`
                (set `self.FirstFloppy` false)
                ;[1 1 1] Sets Current Floppy for reset purposes
                (set `self.Current Floppy` (`self.Other Actor`))
                ;[1 1 1] Check if needs to activate the credits panel
                (bind _asfloppy_text (cast `/Game/Stutter_Speak_Content/Widgets/Floppy_Text` (`WidgetComponent.GetWidget` (`/Game/Stutter_Speak_Content/Blueprints/Floppy.Floppy Name` (`self.Chosen Floppy`)))))
                (if (`KismetStringLibrary.EqualEqual_StrStr` (`/Game/Stutter_Speak_Content/Widgets/Floppy_Text.Orignal Name` _asfloppy_text) "Credits")
                  ;[1 1 1] Changes Details to credits
                  (bind _outactors_10 (`GameplayStatics.GetAllActorsOfClass` "/Game/Stutter_Speak_Content/Blueprints/ProjectorScreen_Blueprint.ProjectorScreen_Blueprint_C"))
                  (bind _asprojector_screen_blueprint_2 (cast `/Game/Stutter_Speak_Content/Blueprints/ProjectorScreen_Blueprint` (`|GetArrayItem` _outactors_10)))
                  (`WidgetComponent.SetWidget` (`/Game/Stutter_Speak_Content/Blueprints/ProjectorScreen_Blueprint.Display` _asprojector_screen_blueprint_2) (`/Game/Stutter_Speak_Content/Blueprints/ProjectorScreen_Blueprint.Credits` _asprojector_screen_blueprint_2))
                  (bind _outactors_11 (`GameplayStatics.GetAllActorsOfClass` "/Game/Stutter_Speak_Content/Blueprints/ResetButton2_Button_Blueprint.ResetButton2_Button_Blueprint_C"))
                  (bind _asreset_button_2_button_blueprint (cast `/Game/Stutter_Speak_Content/Blueprints/ResetButton2_Button_Blueprint` (`|GetArrayItem` _outactors_11)))
                  (set `/Game/Stutter_Speak_Content/Blueprints/ResetButton2_Button_Blueprint.Credits` true _asreset_button_2_button_blueprint)
                  (bind _outactors_12 (`GameplayStatics.GetAllActorsOfClass` "/Game/Stutter_Speak_Content/Pre-Fabs/ResetButton2_Top_Blueprint.ResetButton2_Top_Blueprint_C"))
                  (bind _asreset_button_2_top_blueprint (cast `/Game/Stutter_Speak_Content/Pre-Fabs/ResetButton2_Top_Blueprint` (`|GetArrayItem` _outactors_12)))
                  (`/Game/Stutter_Speak_Content/Pre-Fabs/ResetButton2_Top_Blueprint.ButtonPress` _asreset_button_2_top_blueprint)
                  (set `self.Reset after credits` true)
                  (else
                    ;[1 1 1] Resets widget if credits was last shown
                    (`self.Reset post credits` (`self.Reset after credits`))
                    (bind _outactors_13 (`GameplayStatics.GetAllActorsOfClass` "/Game/Stutter_Speak_Content/Blueprints/ResetButton2_Button_Blueprint.ResetButton2_Button_Blueprint_C"))
                    (bind _asreset_button_2_button_blueprint_2 (cast `/Game/Stutter_Speak_Content/Blueprints/ResetButton2_Button_Blueprint` (`|GetArrayItem` _outactors_13)))
                    (set `/Game/Stutter_Speak_Content/Blueprints/ResetButton2_Button_Blueprint.Credits` false _asreset_button_2_button_blueprint_2)
                    ;[1 1 1] Stores speech name in save data with floppy
                    (bind _asfloppy_text_2 (cast `/Game/Stutter_Speak_Content/Widgets/Floppy_Text` (`WidgetComponent.GetWidget` (`/Game/Stutter_Speak_Content/Blueprints/Floppy.Floppy Name` (`self.Chosen Floppy`)))))
                    (`/Game/Stutter_Speak_Content/Widgets/Floppy_Text.StoreSpeechNameByProjector` _asfloppy_text_2)))
                ;[1 1 1] Projector Screen Fade Out
                (`/Game/Stutter_Speak_Content/Blueprints/ProjectorScreen_Blueprint.ProjectorFadeOut` _asprojector_screen_blueprint)
                (`KismetSystemLibrary.Delay` 0.5)
                (bind _outactors_14 (`GameplayStatics.GetAllActorsOfClass` "/Game/Stutter_Speak_Content/Pre-Fabs/CompleteModels/Projection/projectorcone_Blueprint.projectorcone_Blueprint_C"))
                (bind _asprojectorcone_blueprint_2 (cast `/Game/Stutter_Speak_Content/Pre-Fabs/CompleteModels/Projection/projectorcone_Blueprint` (`|GetArrayItem` _outactors_14)))
                (`/Game/Stutter_Speak_Content/Pre-Fabs/CompleteModels/Projection/projectorcone_Blueprint.Fade in` _asprojectorcone_blueprint_2)
                (`KismetSystemLibrary.Delay` 0.5)
                ;[1 1 1] Enables collision for grab box after animation
                (`PrimitiveComponent.SetCollisionEnabled` (`self.Overlapped Component`) "QueryAndPhysics")
                (bind _asfloppy_text_3 (cast `/Game/Stutter_Speak_Content/Widgets/Floppy_Text` (`WidgetComponent.GetWidget` (`/Game/Stutter_Speak_Content/Blueprints/Floppy.Floppy Name` (`self.Chosen Floppy`)))))
                (if (`KismetStringLibrary.EqualEqual_StrStr` (`/Game/Stutter_Speak_Content/Widgets/Floppy_Text.Orignal Name` _asfloppy_text_3) "Credits")
                  ;[1 1 1] Unhides left and right tab buttons
                  (bind _outactors_15 (`GameplayStatics.GetAllActorsOfClass` "/Game/Stutter_Speak_Content/Pre-Fabs/CompleteModels/LeftButton.LeftButton_C"))
                  (bind _asleft_button (cast `/Game/Stutter_Speak_Content/Pre-Fabs/CompleteModels/LeftButton` (`|GetArrayItem` _outactors_15)))
                  (set `/Game/Stutter_Speak_Content/Pre-Fabs/CompleteModels/LeftButton.ButtonOn` false _asleft_button)
                  (bind _outactors_16 (`GameplayStatics.GetAllActorsOfClass` "/Game/Stutter_Speak_Content/Pre-Fabs/CompleteModels/RightButton.RightButton_C"))
                  (bind _asright_button (cast `/Game/Stutter_Speak_Content/Pre-Fabs/CompleteModels/RightButton` (`|GetArrayItem` _outactors_16)))
                  (set `/Game/Stutter_Speak_Content/Pre-Fabs/CompleteModels/RightButton.ButtonOn` false _asright_button)
                  (bind _outactors_17 (`GameplayStatics.GetAllActorsOfClass` "/Game/Stutter_Speak_Content/Pre-Fabs/CompleteModels/BeginButton.BeginButton_C"))
                  (bind _asbegin_button_2 (cast `/Game/Stutter_Speak_Content/Pre-Fabs/CompleteModels/BeginButton` (`|GetArrayItem` _outactors_17)))
                  (set `/Game/Stutter_Speak_Content/Pre-Fabs/CompleteModels/BeginButton.ButtonOn` false _asbegin_button_2)
                  (bind _outactors_18 (`GameplayStatics.GetAllActorsOfClass` "/Game/Stutter_Speak_Content/Blueprints/ResetButton2_Button_Blueprint.ResetButton2_Button_Blueprint_C"))
                  (bind _asreset_button_2_button_blueprint_3 (cast `/Game/Stutter_Speak_Content/Blueprints/ResetButton2_Button_Blueprint` (`|GetArrayItem` _outactors_18)))
                  (set `/Game/Stutter_Speak_Content/Blueprints/ResetButton2_Button_Blueprint.Button On` false _asreset_button_2_button_blueprint_3)
                  (else
                    ;[1 1 1] Unhides left and right tab buttons
                    (bind _outactors_19 (`GameplayStatics.GetAllActorsOfClass` "/Game/Stutter_Speak_Content/Pre-Fabs/CompleteModels/LeftButton.LeftButton_C"))
                    (bind _asleft_button_2 (cast `/Game/Stutter_Speak_Content/Pre-Fabs/CompleteModels/LeftButton` (`|GetArrayItem` _outactors_19)))
                    (set `/Game/Stutter_Speak_Content/Pre-Fabs/CompleteModels/LeftButton.ButtonOn` true _asleft_button_2)
                    (bind _outactors_20 (`GameplayStatics.GetAllActorsOfClass` "/Game/Stutter_Speak_Content/Pre-Fabs/CompleteModels/RightButton.RightButton_C"))
                    (bind _asright_button_2 (cast `/Game/Stutter_Speak_Content/Pre-Fabs/CompleteModels/RightButton` (`|GetArrayItem` _outactors_20)))
                    (set `/Game/Stutter_Speak_Content/Pre-Fabs/CompleteModels/RightButton.ButtonOn` true _asright_button_2)
                    (bind _outactors_21 (`GameplayStatics.GetAllActorsOfClass` "/Game/Stutter_Speak_Content/Pre-Fabs/CompleteModels/BeginButton.BeginButton_C"))
                    (bind _asbegin_button_3 (cast `/Game/Stutter_Speak_Content/Pre-Fabs/CompleteModels/BeginButton` (`|GetArrayItem` _outactors_21)))
                    (set `/Game/Stutter_Speak_Content/Pre-Fabs/CompleteModels/BeginButton.ButtonOn` true _asbegin_button_3)
                    (bind _outactors_22 (`GameplayStatics.GetAllActorsOfClass` "/Game/Stutter_Speak_Content/Pre-Fabs/ResetButton2_Top_Blueprint.ResetButton2_Top_Blueprint_C"))
                    (bind _asreset_button_2_top_blueprint_2 (cast `/Game/Stutter_Speak_Content/Pre-Fabs/ResetButton2_Top_Blueprint` (`|GetArrayItem` _outactors_22)))
                    (set `/Game/Stutter_Speak_Content/Pre-Fabs/ResetButton2_Top_Blueprint.Grabbable` true _asreset_button_2_top_blueprint_2))))))
          (:`then_1`
            (`/Game/Stutter_Speak_Content/Blueprints/Floppy.EnablePhysicsByProjector` _asfloppy)))
        (else
          (set `self.Not First Time` true)
          (goto _label))))))

(fn `Reset Current Floppy`
  ;[1 1 1] Catches errors on first run
  (if (`self.Not First Time`)
    (bind _outactors (`GameplayStatics.GetAllActorsOfClassWithTag` "/Game/Stutter_Speak_Content/Blueprints/Floppy.Floppy_C" (`|GetArrayItem` (`Actor.Tags` (`self.Current Floppy`)) 1)))
    (bind _asfloppy (cast `/Game/Stutter_Speak_Content/Blueprints/Floppy` (`|GetArrayItem` _outactors)))
    (else
      (set `self.Not First Time` true))))

(fn `Reset post credits`
  (params (`Needs Reset` :type Boolean))
  (if `Needs Reset`
    (bind _outactors (`GameplayStatics.GetAllActorsOfClass` "/Game/Stutter_Speak_Content/Blueprints/ProjectorScreen_Blueprint.ProjectorScreen_Blueprint_C"))
    (bind _asprojector_screen_blueprint (cast `/Game/Stutter_Speak_Content/Blueprints/ProjectorScreen_Blueprint` (`|GetArrayItem` _outactors)))
    (`WidgetComponent.SetWidget` (`/Game/Stutter_Speak_Content/Blueprints/ProjectorScreen_Blueprint.Display` _asprojector_screen_blueprint) (`/Game/Stutter_Speak_Content/Blueprints/ProjectorScreen_Blueprint.Details` _asprojector_screen_blueprint))
    (set `self.Reset after credits` false)))

(fn `UserConstructionScript`)