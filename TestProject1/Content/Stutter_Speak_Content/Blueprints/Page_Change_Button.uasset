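; A pressable page arrow that flips the speech pages shown on the BPSpeechWorld widget, acting as Next or Previous by its first actor tag.
; A HandHit overlap from above dips the arrow, plays a sound and turns the page if MenuGI's PagesArray has a non-empty neighbor.
; Material swaps mark whether each direction is available.
; At start, the Next button hides both buttons when no next page exists.
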(event `self.ReceiveBeginPlay`
  (bind _textrender (`self.TextRender`))
  (bind _textrender_2 (`self.TextRender`))
  (bind _output (`|GetArrayItem` (`self.Tags`)))
  (bind (_relativerotation_roll _relativerotation_pitch _relativerotation_yaw) (`KismetMathLibrary.BreakRotator` (`SceneComponent.RelativeRotation` _textrender)))
  (bind (_relativelocation_x _relativelocation_y _relativelocation_z) (`KismetMathLibrary.BreakVector` (`SceneComponent.RelativeLocation` _textrender_2)))
  (bind _outactors (`GameplayStatics.GetAllActorsOfClass` "/Game/Stutter_Speak_Content/Widgets/BPSpeechWorld.BPSpeechWorld_C"))
  (bind _asbpspeech_world (cast `/Game/Stutter_Speak_Content/Widgets/BPSpeechWorld` (`|GetArrayItem` _outactors)))
  ;[1 1 1] Setting Text Corretly
  (bind _asspeech_page_w (cast `/Game/Stutter_Speak_Content/Widgets/Speech_World/SpeechPageW` (`WidgetComponent.GetWidget` (`/Game/Stutter_Speak_Content/Widgets/BPSpeechWorld.Widget` _asbpspeech_world))))
  (set `self.As Speech Page W` _asspeech_page_w)
  (set `self.TypeTag` _output)
  (if (== _output "Next")
    (`SceneComponent.K2_SetRelativeRotation` _textrender (`KismetMathLibrary.MakeRotator` _relativerotation_roll _relativerotation_pitch (+ _relativerotation_yaw 180.0)) false false)
    (`TextRenderComponent.K2_SetText` (`self.TextRender`) (`self.Next`))
    (`SceneComponent.K2_SetRelativeLocation` _textrender_2 (`KismetMathLibrary.MakeVector` 0.0 _relativelocation_y _relativelocation_z) false false)
    (bind _result (`self.Can Change Page`))
    (if (not _result)
      (`self.SetActorHiddenInGame` true)
      (`PrimitiveComponent.SetCollisionEnabled` (`self.Arrow`) "NoCollision")
      (bind _outactors_2 (`GameplayStatics.GetAllActorsOfClassWithTag` "Page_Change_Button_C" "Back"))
      (bind _aspage_change_button (cast `/Game/Stutter_Speak_Content/Blueprints/Page_Change_Button` (`|GetArrayItem` _outactors_2)))
      (`self.SetActorHiddenInGame` _aspage_change_button true)
      (`PrimitiveComponent.SetCollisionEnabled` (`/Game/Stutter_Speak_Content/Blueprints/Page_Change_Button.Arrow` _aspage_change_button) "NoCollision"))
    (else
      (`TextRenderComponent.K2_SetText` (`self.TextRender`) (`self.Previous`))
      (`PrimitiveComponent.SetMaterial` (`self.Arrow`) 0 "/Game/Stutter_Speak_Content/Materials/MenuWorldMiscMaterials/SettingsBox.SettingsBox")
      (`PrimitiveComponent.SetMaterial` (`self.Arrow`) 1 "/Game/Stutter_Speak_Content/Materials/MenuWorldMiscMaterials/SettingsBox.SettingsBox"))))

(event `self.Arrow.OnComponentBeginOverlap`
  (params (OverlappedComponent :type "PrimitiveComponent Object Reference") (OtherActor :type "Actor Object Reference") (OtherComp :type "PrimitiveComponent Object Reference") (OtherBodyIndex :type Integer) (bFromSweep :type Boolean) (SweepResult :type "HitResult Structure (by ref)"))
  (bind (_returnvalue_x _returnvalue_y _returnvalue_z) (`KismetMathLibrary.BreakVector` (`SceneComponent.K2_GetComponentLocation` OtherComp)))
  (bind _sound (`self.Sound`))
  (bind _arrow (`self.Arrow`))
  (bind _as_speech_page_w (`self.As Speech Page W`))
  (bind (_returnvalue_x_2 _returnvalue_y_2 _returnvalue_z_2) (`KismetMathLibrary.BreakVector` (`SceneComponent.K2_GetComponentLocation` (`self.Arrow`))))
  (bind (_returnvalue_location _returnvalue_rotation _returnvalue_scale) (`KismetMathLibrary.BreakTransform` (`SceneComponent.GetRelativeTransform` (`self.Arrow`))))
  ;[1 1 1] Conditions for Functioning
  (if (`self.Active`)
    (if (> _returnvalue_z _returnvalue_z_2)
      (if (`KismetStringLibrary.EqualEqual_StrStr` (`KismetSystemLibrary.GetObjectName` OtherComp) "HandHit")
        (if (not (`self.isPressedDown`))
          (bind _result (`self.Can Change Page`))
          (if _result
            ;[1 1 1] Moves Button Top
            (bind _output_get (set `self.Up Location` _returnvalue_location))
            (set `self.Return Value Rotation` _returnvalue_rotation)
            (set `self.Return Value Scale` _returnvalue_scale)
            (`SceneComponent.K2_SetRelativeTransform` (`self.Arrow`) (`KismetMathLibrary.MakeTransform` (- _output_get (0.0 0.0 2.0)) (`self.Return Value Rotation`) (`self.Return Value Scale`)) false false)
            ;[1 1 1] Playing Audio
            (`AudioComponent.SetPitchMultiplier` _sound 1.25)
            (`AudioComponent.Play` _sound 0.0)
            (set `self.isPressedDown` true)
            ;[1 1 1] Updates Page Accordingly
            (if (== (`|GetArrayItem` (`self.Tags`)) "Next")
              (`/Game/Stutter_Speak_Content/Widgets/Speech_World/SpeechPageW.NextPageByNextButton` _as_speech_page_w)
              (else
                (`/Game/Stutter_Speak_Content/Widgets/Speech_World/SpeechPageW.PreviousPageByBackButton` _as_speech_page_w)))
            (`KismetSystemLibrary.Delay` 0.2)
            ;[1 1 1] Released
            (if (`self.isPressedDown`)
              (`SceneComponent.K2_SetRelativeTransform` (`self.Arrow`) (`KismetMathLibrary.MakeTransform` (`self.Up Location`) (`self.Return Value Rotation`) (`self.Return Value Scale`)) false false)
              (set `self.isPressedDown` false)
              (bind _result_2 (`self.Can Change Page`))
              (if (not _result_2)
                (`PrimitiveComponent.SetMaterial` _arrow 0 "/Game/Stutter_Speak_Content/Materials/MenuWorldMiscMaterials/SettingsBox.SettingsBox")
                (`PrimitiveComponent.SetMaterial` _arrow 1 "/Game/Stutter_Speak_Content/Materials/MenuWorldMiscMaterials/SettingsBox.SettingsBox"))
              (if (== (`self.TypeTag`) "Next")
                (bind _outactors (`GameplayStatics.GetAllActorsOfClassWithTag` "Page_Change_Button_C" "Back"))
                (bind _aspage_change_button (cast `/Game/Stutter_Speak_Content/Blueprints/Page_Change_Button` (`|GetArrayItem` _outactors)))
                (bind _arrow_2 (`/Game/Stutter_Speak_Content/Blueprints/Page_Change_Button.Arrow` _aspage_change_button))
                (`PrimitiveComponent.SetMaterial` _arrow_2 0 "/Game/Stutter_Speak_Content/Materials/MenuBG.MenuBG")
                (`PrimitiveComponent.SetMaterial` _arrow_2 1 "/Game/Stutter_Speak_Content/Materials/MenuBG.MenuBG")
                (else
                  (bind _outactors_2 (`GameplayStatics.GetAllActorsOfClassWithTag` "Page_Change_Button_C" "Next"))
                  (bind _aspage_change_button_2 (cast `/Game/Stutter_Speak_Content/Blueprints/Page_Change_Button` (`|GetArrayItem` _outactors_2)))
                  (bind _arrow_3 (`/Game/Stutter_Speak_Content/Blueprints/Page_Change_Button.Arrow` _aspage_change_button_2))
                  (`PrimitiveComponent.SetMaterial` _arrow_3 0 "/Game/Stutter_Speak_Content/Materials/MenuBG.MenuBG")
                  (`PrimitiveComponent.SetMaterial` _arrow_3 1 "/Game/Stutter_Speak_Content/Materials/MenuBG.MenuBG"))))))))))

(fn `Can Change Page`
  (returns (Result :type Boolean))
  (if (== (`|GetArrayItem` (`self.Tags`)) "Next")
    (bind _asmenu_gi (cast `/Game/Stutter_Speak_Content/Blueprints/MenuGI` (`GameplayStatics.GetGameInstance`)))
    (if (`KismetStringLibrary.NotEqual_StrStr` (`|GetArrayItem` (`/Game/Stutter_Speak_Content/Blueprints/MenuGI.PagesArray` _asmenu_gi) (+ (`/Game/Stutter_Speak_Content/Widgets/Speech_World/SpeechPageW.PageNum` (`self.As Speech Page W`)) 1)))
      _
      (else
        (return false)))
    (else
      (bind _asmenu_gi_2 (cast `/Game/Stutter_Speak_Content/Blueprints/MenuGI` (`GameplayStatics.GetGameInstance`)))
      (if (`KismetStringLibrary.NotEqual_StrStr` (`|GetArrayItem` (`/Game/Stutter_Speak_Content/Blueprints/MenuGI.PagesArray` _asmenu_gi_2) (- (`/Game/Stutter_Speak_Content/Widgets/Speech_World/SpeechPageW.PageNum` (`self.As Speech Page W`)) 1)))
        _
        (else
          (return false)))))
  (return true))

(fn `UserConstructionScript`)