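; Projector screen actor that hosts a details widget and fades a projector overlay mesh in and out.
; On BeginPlay it hides the Display widget, creates and stores a Credits widget, and applies a dynamic material to ProjectorFader.
; An event reveals the details, while fade events use timelines to drive the material's Opacity.
; Fade-in plays in reverse and, while Condition is false, only sets that flag instead of animating.
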(event `self.ReceiveBeginPlay`
  (`Widget.SetVisibility` (`WidgetComponent.GetWidget` (`self.Display`)) "Hidden")
  (set `self.Details` (`WidgetComponent.GetWidget` (`self.Display`)))
  (bind _returnvalue (`|CreateWidget` "/Game/Stutter_Speak_Content/Widgets/Menu_World_Widgets/Credits.Credits_C"))
  (set `self.Credits` _returnvalue)
  (bind _returnvalue_2 (`KismetMaterialLibrary.CreateDynamicMaterialInstance` "/Game/Stutter_Speak_Content/Materials/ProjectorMaterials/Screen/Projector_Screen_Secondary.Projector_Screen_Secondary"))
  (bind _output_get (set `self.MAT` _returnvalue_2))
  (`PrimitiveComponent.SetMaterial` (`self.ProjectorFader`) 0 _output_get))

(event `ShowDetailsByDetailsPanel`
  (`Widget.SetVisibility` (`WidgetComponent.GetWidget` (`self.Display`)) "Visible"))

(event `ProjectorFadeIn`
  (if (`self.Condition`)
    (bind (_direction _newtrack_0) (`Timeline|Timeline_1` :!via `ReverseFromEnd`)
      (:`Update`
        (`MaterialInstanceDynamic.SetScalarParameterValue` (`self.MAT`) "Opacity" _newtrack_0)))
    (else
      (set `self.Condition` true))))

(event `ProjectorFadeOut`
  (bind (_direction _newtrack_0) (`Timeline|Timeline_0` :!via `PlayFromStart`)
    (:`Update`
      (`MaterialInstanceDynamic.SetScalarParameterValue` (`self.MAT`) "Opacity" _newtrack_0))))

(fn `UserConstructionScript`)