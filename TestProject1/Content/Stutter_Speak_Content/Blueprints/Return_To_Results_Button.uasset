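; A physical VR button that ends retracking and returns the player to the results display.
; It starts hidden, rises when RaiseButton is called, and responds to a HandHit overlap from above with a brief press and click sound.
; On release it clears motion-controller retracking, stops and clears the stutter timer, and resets Pause/Play.
; It then lowers itself, shows results on the projector screen, and raises the Menu, Retry and Retrack buttons.
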(event `self.ReceiveBeginPlay`
  ;[1 1 1] Hides Button at the Start
  (`self.SetActorHiddenInGame` true))

(event `self.Retrack Button.OnComponentBeginOverlap`
  (params (OverlappedComponent :type "PrimitiveComponent Object Reference") (OtherActor :type "Actor Object Reference") (OtherComp :type "PrimitiveComponent Object Reference") (OtherBodyIndex :type Integer) (bFromSweep :type Boolean) (SweepResult :type "HitResult Structure (by ref)"))
  (bind (_returnvalue_x _returnvalue_y _returnvalue_z) (`KismetMathLibrary.BreakVector` (`SceneComponent.K2_GetComponentLocation` OtherComp)))
  (bind _sound (`self.Sound`))
  (bind (_returnvalue_x_2 _returnvalue_y_2 _returnvalue_z_2) (`KismetMathLibrary.BreakVector` (`SceneComponent.K2_GetComponentLocation` (`self.Retrack Button`))))
  (bind (_returnvalue_location _returnvalue_rotation _returnvalue_scale) (`KismetMathLibrary.BreakTransform` (`SceneComponent.GetRelativeTransform` (`self.Retrack Button`))))
  ;[1 1 1] Conditions for Functioning
  (if (`self.Active`)
    (set `self.Active` false)
    (if (> _returnvalue_z _returnvalue_z_2)
      (if (`KismetStringLibrary.EqualEqual_StrStr` (`KismetSystemLibrary.GetObjectName` OtherComp) "HandHit")
        (if (not (`self.isPressedDown`))
          ;[1 1 1] Moves Button Top
          (bind _output_get (set `self.Up Location` _returnvalue_location))
          (set `self.Return Value Rotation` _returnvalue_rotation)
          (set `self.Return Value Scale` _returnvalue_scale)
          (`SceneComponent.K2_SetRelativeTransform` (`self.Retrack Button`) (`KismetMathLibrary.MakeTransform` (- _output_get (0.0 0.0 0.5)) (`self.Return Value Rotation`) (`self.Return Value Scale`)) false false)
          ;[1 1 1] Playing Audio
          (`AudioComponent.SetPitchMultiplier` _sound 0.75)
          (`AudioComponent.Play` _sound 0.0)
          (set `self.isPressedDown` true)
          ;[1 1 1] Released
          (`KismetSystemLibrary.Delay` 0.2)
          (if (`self.isPressedDown`)
            (`SceneComponent.K2_SetRelativeTransform` (`self.Retrack Button`) (`KismetMathLibrary.MakeTransform` (`self.Up Location`) (`self.Return Value Rotation`) (`self.Return Value Scale`)) false false)
            (set `self.isPressedDown` false)
            (bind _outactors (`GameplayStatics.GetAllActorsOfClass` "/Game/Starter_Content/VirtualRealityBP/Blueprints/BP_MotionController.BP_MotionController_C"))
            (for (_ _array_index) _outactors
              (bind _asbp_motion_controller (cast `/Game/Starter_Content/VirtualRealityBP/Blueprints/BP_MotionController` (`|GetArrayItem` _outactors _array_index)))
              (set `/Game/Starter_Content/VirtualRealityBP/Blueprints/BP_MotionController.Retracking` false _asbp_motion_controller))
            (bind _outactors_2 (`GameplayStatics.GetAllActorsOfClass` "/Game/Stutter_Speak_Content/Managers/Stutter_Timer__Empty_Object__Blueprint.Stutter_Timer__Empty_Object__Blueprint_C"))
            (bind _asstutter_timer__empty_object__blueprint (cast `/Game/Stutter_Speak_Content/Managers/Stutter_Timer__Empty_Object__Blueprint` (`|GetArrayItem` _outactors_2)))
            (`/Game/Stutter_Speak_Content/Managers/Stutter_Timer__Empty_Object__Blueprint.Stop Timer` _asstutter_timer__empty_object__blueprint)
            (`/Game/Stutter_Speak_Content/Managers/Stutter_Timer__Empty_Object__Blueprint.ClearData` _asstutter_timer__empty_object__blueprint)
            (bind _outactors_3 (`GameplayStatics.GetAllActorsOfClass` "/Game/Stutter_Speak_Content/Blueprints/Pause_Play_Button.Pause_Play_Button_C"))
            (bind _aspause_play_button (cast `/Game/Stutter_Speak_Content/Blueprints/Pause_Play_Button` (`|GetArrayItem` _outactors_3)))
            (`/Game/Stutter_Speak_Content/Blueprints/Pause_Play_Button.ForceStop` _aspause_play_button)
            (set `/Game/Stutter_Speak_Content/Blueprints/Pause_Play_Button.Active_Play` false _aspause_play_button)
            (set `/Game/Stutter_Speak_Content/Blueprints/Pause_Play_Button.Active_Pause` false _aspause_play_button)
            (`/Game/Stutter_Speak_Content/Blueprints/Pause_Play_Button.Reset` _aspause_play_button)
            (`/Game/Stutter_Speak_Content/Blueprints/Pause_Play_Button.Lower Button` _aspause_play_button)
            (`self.Lower Button`)
            (bind _outactors_4 (`GameplayStatics.GetAllActorsOfClass` "/Game/Stutter_Speak_Content/Blueprints/Hanging_Projector_Screen_Blueprint.Hanging_Projector_Screen_Blueprint_C"))
            (bind _ashanging_projector_screen_blueprint (cast `/Game/Stutter_Speak_Content/Blueprints/Hanging_Projector_Screen_Blueprint` (`|GetArrayItem` _outactors_4)))
            (`/Game/Stutter_Speak_Content/Blueprints/Hanging_Projector_Screen_Blueprint.DisplayResults` _ashanging_projector_screen_blueprint)
            ;[1 1 1] Rasing Menu, Retry, & Retrack Buttons
            (bind _outactors_5 (`GameplayStatics.GetAllActorsOfClass` "/Game/Stutter_Speak_Content/Blueprints/Menu_Button.Menu_Button_C"))
            (bind _asmenu_button (cast `/Game/Stutter_Speak_Content/Blueprints/Menu_Button` (`|GetArrayItem` _outactors_5)))
            (`/Game/Stutter_Speak_Content/Blueprints/Menu_Button.RaiseButton` _asmenu_button)
            (bind _outactors_6 (`GameplayStatics.GetAllActorsOfClass` "/Game/Stutter_Speak_Content/Blueprints/Retry_Button.Retry_Button_C"))
            (bind _asretry_button (cast `/Game/Stutter_Speak_Content/Blueprints/Retry_Button` (`|GetArrayItem` _outactors_6)))
            (`/Game/Stutter_Speak_Content/Blueprints/Retry_Button.RaiseButton` _asretry_button)
            (bind _outactors_7 (`GameplayStatics.GetAllActorsOfClass` "/Game/Stutter_Speak_Content/Blueprints/Retrack.Retrack_C"))
            (bind _asretrack (cast `/Game/Stutter_Speak_Content/Blueprints/Retrack` (`|GetArrayItem` _outactors_7)))
            (`/Game/Stutter_Speak_Content/Blueprints/Retrack.RaiseButton` _asretrack)
            (`PrimitiveComponent.SetMaterial` (`/Game/Stutter_Speak_Content/Blueprints/Menu_Button.Menu Button` _asmenu_button) 0 "/Game/Starter_Content/VirtualReality/Materials/M_BaseMaterial.M_BaseMaterial")
            (`PrimitiveComponent.SetMaterial` (`/Game/Stutter_Speak_Content/Blueprints/Retry_Button.Retry Button` _asretry_button) 0 "/Game/Starter_Content/VirtualReality/Materials/M_BaseMaterial.M_BaseMaterial")
            (`PrimitiveComponent.SetMaterial` (`/Game/Stutter_Speak_Content/Blueprints/Retrack.Retrack Button` _asretrack) 0 "/Game/Starter_Content/VirtualReality/Materials/M_BaseMaterial.M_BaseMaterial")))))))

(event `RaiseButton`
  (bind _defaultsceneroot (`self.DefaultSceneRoot`))
  ;[1 1 1] Raises Button When Called
  (`self.SetActorHiddenInGame` false)
  (`KismetSystemLibrary.MoveComponentTo` _defaultsceneroot (+ (`SceneComponent.RelativeLocation` _defaultsceneroot) (0.0 0.0 7.5)) (`SceneComponent.RelativeRotation` _defaultsceneroot) false false 1.0)
  (set `self.Active` true))

(event `Lower Button`
  (bind _defaultsceneroot (`self.DefaultSceneRoot`))
  ;[1 1 1] Lower Button When Called
  (set `self.Active` false)
  (`KismetSystemLibrary.MoveComponentTo` _defaultsceneroot (+ (`SceneComponent.RelativeLocation` _defaultsceneroot) (0.0 0.0 -7.5)) (`SceneComponent.RelativeRotation` _defaultsceneroot) false false 1.0)
  (`self.SetActorHiddenInGame` true))

(fn `UserConstructionScript`)