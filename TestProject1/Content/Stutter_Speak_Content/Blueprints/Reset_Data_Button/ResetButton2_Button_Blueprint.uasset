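; Physical reset button that deletes speech data through MenuGI when pressed from above by a HandHit component, outside of Credits.
; An overlap lowers the mesh, plays a pitched-down sound and triggers CancelByReset on Cancel_BP.
; After a short delay the mesh rises, then Projector_Blueprint fades in and ResetButton2_Top_Blueprint receives ButtonPress.
; ButtonOn clears on the first overlap, before the height and name checks, and is never re-armed here.
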(event `self.StaticMeshComponent.OnComponentBeginOverlap`
  (params (OverlappedComponent :type "PrimitiveComponent Object Reference") (OtherActor :type "Actor Object Reference") (OtherComp :type "PrimitiveComponent Object Reference") (OtherBodyIndex :type Integer) (bFromSweep :type Boolean) (SweepResult :type "HitResult Structure (by ref)"))
  (bind (_returnvalue_x _returnvalue_y _returnvalue_z) (`KismetMathLibrary.BreakVector` (`SceneComponent.K2_GetComponentLocation` OtherComp)))
  (bind _audio (`self.Audio`))
  (bind (_returnvalue_x_2 _returnvalue_y_2 _returnvalue_z_2) (`KismetMathLibrary.BreakVector` (`SceneComponent.K2_GetComponentLocation` (`self.StaticMeshComponent`))))
  (bind _returnvalue (`SceneComponent.GetRelativeTransform` (`self.StaticMeshComponent`)))
  (bind _returnvalue_2 (`SceneComponent.GetRelativeTransform` (`self.StaticMeshComponent`)))
  (if (not (`self.Credits`))
    ;[1 1 1] Pressed Down
    (if (`self.Button On`)
      (set `self.Button On` false)
      (if (> _returnvalue_z _returnvalue_z_2)
        (if (`KismetStringLibrary.EqualEqual_StrStr` (`KismetSystemLibrary.GetObjectName` OtherComp) "HandHit")
          (`SceneComponent.K2_SetRelativeTransform` (`self.StaticMeshComponent`) (`KismetMathLibrary.MakeTransform` (`KismetMathLibrary.MakeVector` (.x (.location _returnvalue_2)) (.y (.location _returnvalue_2)) (- (.z (.location _returnvalue_2)) 3.0)) (.rotation _returnvalue_2) (.scale _returnvalue_2)) false false)
          (`AudioComponent.SetPitchMultiplier` _audio 0.75)
          (`AudioComponent.Play` _audio 0.0)
          (bind _asmenu_gi (cast `/Game/Stutter_Speak_Content/Blueprints/MenuGI` (`GameplayStatics.GetGameInstance`)))
          (`/Game/Stutter_Speak_Content/Blueprints/MenuGI.DeleteSpeechDataByResetButton` _asmenu_gi)
          (bind _outactors (`GameplayStatics.GetAllActorsOfClass` "/Game/Stutter_Speak_Content/Blueprints/Cancel_BP.Cancel_BP_C"))
          (bind _ascancel_bp (cast `/Game/Stutter_Speak_Content/Blueprints/Cancel_BP` (`|GetArrayItem` _outactors)))
          (`/Game/Stutter_Speak_Content/Blueprints/Cancel_BP.CancelByReset` _ascancel_bp)
          (`KismetSystemLibrary.Delay` 0.35)
          ;[1 1 1] Released
          (`SceneComponent.K2_SetRelativeTransform` (`self.StaticMeshComponent`) (`KismetMathLibrary.MakeTransform` (`KismetMathLibrary.MakeVector` (.x (.location _returnvalue)) (.y (.location _returnvalue)) (+ (.z (.location _returnvalue)) 3.0)) (.rotation _returnvalue) (.scale _returnvalue)) false false)
          (bind _outactors_2 (`GameplayStatics.GetAllActorsOfClass` "/Game/Stutter_Speak_Content/Blueprints/Projector_Blueprint.Projector_Blueprint_C"))
          (bind _asprojector_blueprint (cast `/Game/Stutter_Speak_Content/Blueprints/Projector_Blueprint` (`|GetArrayItem` _outactors_2)))
          (`/Game/Stutter_Speak_Content/Blueprints/Projector_Blueprint.FadeInOnReset` _asprojector_blueprint)
          (bind _outactors_3 (`GameplayStatics.GetAllActorsOfClass` "/Game/Stutter_Speak_Content/Pre-Fabs/ResetButton2_Top_Blueprint.ResetButton2_Top_Blueprint_C"))
          (bind _asreset_button_2_top_blueprint (cast `/Game/Stutter_Speak_Content/Pre-Fabs/ResetButton2_Top_Blueprint` (`|GetArrayItem` _outactors_3)))
          (`/Game/Stutter_Speak_Content/Pre-Fabs/ResetButton2_Top_Blueprint.ButtonPress` _asreset_button_2_top_blueprint))))))

(fn `UserConstructionScript`)