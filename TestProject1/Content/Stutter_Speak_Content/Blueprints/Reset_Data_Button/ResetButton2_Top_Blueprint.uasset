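; Hinged top of a reset button that toggles between two positions when picked up, arming or disarming the button.
; A FlipFlop plays the MoveTop timeline forward or in reverse, driving the pitch of the mesh's parent component.
; Grabbable blocks further pickups during the motion.
; On finish, it sets ButtonOn on the first ResetButton2_Button_Blueprint in the level to match the toggle state.
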(event `/Game/Starter_Content/VirtualRealityBP/Blueprints/PickupActorInterface.Pickup`
  (params (AttachTo :type "SceneComponent Object Reference"))
  (if (`self.Grabbable`)
    (set `self.Grabbable` false)
    (bind _isa (`/Engine/EditorBlueprintResources/StandardMacros.FlipFlop`)
      (:`A`
        (bind (_direction _newtrack_0) (`Timeline|MoveTop` :!via `PlayFromStart` :!label _label)
          (:`Update`
            (`SceneComponent.K2_SetWorldRotation` (`SceneComponent.GetAttachParent` (`self.StaticMeshComponent`)) (`KismetMathLibrary.MakeRotator` 0.0 (* _newtrack_0 (`self.MovementVar`)) 30.0) false false))
          (:`Finished`
            (set `self.Grabbable` true)
            (bind _outactors (`GameplayStatics.GetAllActorsOfClass` "/Game/Stutter_Speak_Content/Blueprints/Reset_Data_Button/ResetButton2_Button_Blueprint.ResetButton2_Button_Blueprint_C"))
            (bind _asreset_button_2_button_blueprint (cast `/Game/Stutter_Speak_Content/Blueprints/Reset_Data_Button/ResetButton2_Button_Blueprint` (`|GetArrayItem` _outactors)))
            (if _isa
              (set `/Game/Stutter_Speak_Content/Blueprints/Reset_Data_Button/ResetButton2_Button_Blueprint.Button On` true _asreset_button_2_button_blueprint)
              (else
                (set `/Game/Stutter_Speak_Content/Blueprints/Reset_Data_Button/ResetButton2_Button_Blueprint.Button On` false _asreset_button_2_button_blueprint))))))
      (:`B`
        (goto _label :!via `ReverseFromEnd`)))))

(fn `UserConstructionScript`)