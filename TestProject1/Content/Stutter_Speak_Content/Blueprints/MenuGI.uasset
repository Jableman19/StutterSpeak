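; Game instance that saves and loads speech attempt records, including stutter time and ratings, for a stuttering speech game.
; Saving triggers the stutter timer's total, then asynchronously reloads one SaveData slot and appends the attempt under its speech name, adding a group if none matches.
; Loading copies the selected speech's attempts, creating the save if needed, and refreshes the speech details widget.
; The next attempt number derives from that copied list's length.
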(event `self.ReceiveInit`
  ;[1 1 1] Creates Necessary Variables on Begin Play
  (set `self.PagesArray` (`|MakeArray` "")))

(event `Call Saving Data`
  (bind _all_saved_data (`/Game/Stutter_Speak_Content/SaveData.All_Saved_Data` (`self.Loaded Data to Overwrite`)))
  ;[1 1 1] Saving Data
  ;;[1 1 1] Collecting all necesary data
  (bind _outactors (`GameplayStatics.GetAllActorsOfClass` "/Game/Stutter_Speak_Content/Blueprints/Stutter_Timer__Empty_Object__Blueprint.Stutter_Timer__Empty_Object__Blueprint_C"))
  (bind _asstutter_timer__empty_object__blueprint (cast `/Game/Stutter_Speak_Content/Blueprints/Stutter_Timer__Empty_Object__Blueprint` (`|GetArrayItem` _outactors)))
  (`/Game/Stutter_Speak_Content/Blueprints/Stutter_Timer__Empty_Object__Blueprint.Get Total Stutter Time` _asstutter_timer__empty_object__blueprint)
  (set `self.Data to Save` (make `/Game/Stutter_Speak_Content/Structs/Attempt_Struct` (`self.Data to Save : Speech Name`) (`self.Data to Save : Attempt #`) (`self.Data to Save : Total Time Taken`) (`self.Data to Save : Total Time Stuttering`) (`self.Data to Save : Audience Looking %`) (`self.Data to Save : Message Satisfacation Rating`) (`self.Data to Save : Fluency Satisfaction Rating`)))
  ;;[1 1 1] Loading in previous data to overwrite and re-save
  (bind _savegame (`AsyncActionHandleSaveGame.AsyncLoadGameFromSlot` "Theoretically")
    (:`Completed`
      (bind _assave_data (cast `/Game/Stutter_Speak_Content/SaveData` _savegame))
      (bind _output_get (set `self.Loaded Data to Overwrite` _assave_data))
      (for (_array_element _array_index) (`/Game/Stutter_Speak_Content/SaveData.All_Saved_Data` _output_get)
        ;;[1 1 1] If match found to existing data, add to that subarray, break loop
        (if (`KismetStringLibrary.EqualEqual_StrStr` (`self.Data to Save : Speech Name`) (break `/Game/Stutter_Speak_Content/Structs/Data_For_Each_Speech_Struct` _array_element))
          (set `self.Match_Found_To_Save_Data` true)
          (bind (_output_speechname _output_saveddataforspeechname) (break `/Game/Stutter_Speak_Content/Structs/Data_For_Each_Speech_Struct` (`|GetArrayItem` (`/Game/Stutter_Speak_Content/SaveData.All_Saved_Data` (`self.Loaded Data to Overwrite`)) _array_index)))
          (`KismetArrayLibrary.Array_Set` _output_saveddataforspeechname (`KismetArrayLibrary.Array_Length` _output_saveddataforspeechname) (`self.Data to Save`) true)
          (break)))
      (if (not (`self.Match_Found_To_Save_Data`))
        (`KismetSystemLibrary.PrintString` "no array found")
        ;;[1 1 1] If no existing data can be found, adds new speech array and adds new element to that subarray
        (bind _returnvalue (`KismetArrayLibrary.Array_Add` _all_saved_data))
        (bind (_output_speechname_2 _output_saveddataforspeechname_2) (break `/Game/Stutter_Speak_Content/Structs/Data_For_Each_Speech_Struct` (`|GetArrayItem` _all_saved_data _returnvalue)))
        (`|VariableSetRef` _output_speechname_2 (`self.Data to Save : Speech Name`))
        (`KismetArrayLibrary.Array_Add` _output_saveddataforspeechname_2 (`self.Data to Save`)))
      (set `self.Match_Found_To_Save_Data` false)
      ;;[1 1 1] Creates new save game object, adds the necessary data, and saves that object
      (bind (_savegame_2 _bsuccess) (`AsyncActionHandleSaveGame.AsyncSaveGameToSlot` (`self.Loaded Data to Overwrite`) "Theoretically")
        (:`Completed`
          (if _bsuccess
            (`KismetSystemLibrary.PrintString` "Game Saved" true true (struct :`G` 0.66 :`B` 1.0 :`A` 1.0) 30.0)))))))

(event `MenuGIDataLoadedByTextButton`
  ;[1 1 1] Loads the save game slot, loops through array to find matching speech names, copies those into seperate array
  (`KismetArrayLibrary.Array_Clear` (`self.Attempts of Selected Speech`))
  (bind _savegame (`AsyncActionHandleSaveGame.AsyncLoadGameFromSlot` "Theoretically")
    (:`Completed`
      (bind _assave_data (cast `/Game/Stutter_Speak_Content/SaveData` _savegame)
        (:`then`
          (set `self.Data to Load` _assave_data))
        (:`CastFailed`
          (bind _returnvalue (`GameplayStatics.CreateSaveGameObject` "/Game/Stutter_Speak_Content/SaveData.SaveData_C"))
          (`AsyncActionHandleSaveGame.AsyncSaveGameToSlot` _returnvalue "Theoretically"
            (:`Completed`
              (bind _savegame_2 (`AsyncActionHandleSaveGame.AsyncLoadGameFromSlot` "Theoretically")
                (:`Completed`
                  (bind _assave_data_2 (cast `/Game/Stutter_Speak_Content/SaveData` _savegame_2))
                  (set `self.Data to Load` _assave_data_2)))))))
      (for _array_element (`/Game/Stutter_Speak_Content/SaveData.All_Saved_Data` (`self.Data to Load`))
        (if (`KismetStringLibrary.EqualEqual_StrStr` (break `/Game/Stutter_Speak_Content/Structs/Data_For_Each_Speech_Struct` _array_element) (`self.Data to Save : Speech Name`))
          (set `self.Match_Found_To_Load_Data` true)
          (for _array_element_2 (`.SavedDataforSpeechName_11_BAF45FEB4E5277F0FF11AEBAA51C1ECC` (break `/Game/Stutter_Speak_Content/Structs/Data_For_Each_Speech_Struct` _array_element))
            (`KismetArrayLibrary.Array_Add` (`self.Attempts of Selected Speech`) _array_element_2))
          (break)))
      (bind _outactors (`GameplayStatics.GetAllActorsOfClass` "/Game/Stutter_Speak_Content/Widgets/BPSpeechDetails.BPSpeechDetails_C"))
      (bind _asbpspeech_details (cast `/Game/Stutter_Speak_Content/Widgets/BPSpeechDetails` (`|GetArrayItem` _outactors)))
      (bind _asspeech_details_pannel (cast `/Game/Stutter_Speak_Content/Widgets/Menu_World_Widgets/Speech_Details_Pannel` (`WidgetComponent.GetWidget` (`/Game/Stutter_Speak_Content/Widgets/BPSpeechDetails.Widget` _asbpspeech_details))))
      (if (`self.Match_Found_To_Load_Data`)
        (`/Game/Stutter_Speak_Content/Widgets/Menu_World_Widgets/Speech_Details_Pannel.CalculateDetailsByMenuGi` _asspeech_details_pannel)
        (`/Game/Stutter_Speak_Content/Widgets/Menu_World_Widgets/Speech_Details_Pannel.SetSpeechNameByMenuGI` _asspeech_details_pannel)
        (else
          (`/Game/Stutter_Speak_Content/Widgets/Menu_World_Widgets/Speech_Details_Pannel.SetSpeechNameByMenuGI` _asspeech_details_pannel))))))

(event `SetAttemptNumberByStartSpeech`
  (bind _returnvalue (`KismetArrayLibrary.Array_Length` (`self.Attempts of Selected Speech`)))
  ;[1 1 1] Gets the number of objects in the array and sets next attempt # +1
  (if (== _returnvalue 0)
    (set `self.Data to Save : Attempt #` 1)
    (else
      (set `self.Data to Save : Attempt #` (+ _returnvalue 1)))))