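; Podium actor for a VR speaking experience that fits its height to the player's headset camera.
; Shortly after BeginPlay it finds the MotionControllerPawn and sets its own Z to a fixed offset below that camera, keeping X and Y.
; A custom event, named for the Level Blueprint to call, instantly drops the podium out of the way for the post-speech phase.
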(event `self.ReceiveBeginPlay`
  (bind (_returnvalue_x _returnvalue_y) (`KismetMathLibrary.BreakVector` (`self.K2_GetActorLocation`)))
  (`KismetSystemLibrary.Delay` 0.2)
  (bind _outactors (`GameplayStatics.GetAllActorsOfClass` "/Game/Starter_Content/VirtualRealityBP/Blueprints/MotionControllerPawn.MotionControllerPawn_C"))
  (bind _asmotion_controller_pawn (cast `/Game/Starter_Content/VirtualRealityBP/Blueprints/MotionControllerPawn` (`|GetArrayItem` _outactors)))
  (bind (_returnvalue_x_2 _returnvalue_y_2 _returnvalue_z) (`KismetMathLibrary.BreakVector` (`SceneComponent.K2_GetComponentLocation` (`/Game/Starter_Content/VirtualRealityBP/Blueprints/MotionControllerPawn.Camera` _asmotion_controller_pawn))))
  (`self.K2_SetActorLocation` (`KismetMathLibrary.MakeVector` _returnvalue_x _returnvalue_y (- _returnvalue_z 175.0))))

(event `RemovePodiumByLevelBlueprint`
  ;[1 1 1] Moves Podium Down for Post Speech
  (`SceneComponent.K2_SetWorldLocation` (`self.DefaultSceneRoot`) (- (`self.K2_GetActorLocation`) (0.0 0.0 300.0)) false false))

(fn `UserConstructionScript`)