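; StopButton is a physical push button that ends a speech recording and brings up the rating interface.
; Tick keeps collision off while hidden, then enables collision and the button one second after it is shown.
; Any hitbox overlap while enabled stops Recording_Test and reveals BPRater, but only overlaps from above depress the top and play audio.
; Releasing a depressed button raises it, clears SpeechOn on MotionControllerPawn and destroys the actor.
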(event `self.ReceiveTick`
  (params (DeltaSeconds :type "Float (single-precision)"))
  (if (`self.bHidden`)
    (`self.SetActorEnableCollision` false)
    (else
      (`KismetSystemLibrary.Delay` 1.0)
      (`self.SetActorEnableCollision` true)
      (set `self.enabled` true))))

(event `self.Hitbox.OnComponentBeginOverlap`
  (params (OverlappedComponent :type "PrimitiveComponent Object Reference") (OtherActor :type "Actor Object Reference") (OtherComp :type "PrimitiveComponent Object Reference") (OtherBodyIndex :type Integer) (bFromSweep :type Boolean) (SweepResult :type "HitResult Structure (by ref)"))
  (bind (_returnvalue_x _returnvalue_y _returnvalue_z) (`KismetMathLibrary.BreakVector` (`SceneComponent.K2_GetComponentLocation` OtherComp)))
  (bind (_returnvalue_x_2 _returnvalue_y_2 _returnvalue_z_2) (`KismetMathLibrary.BreakVector` (`SceneComponent.K2_GetComponentLocation` (`self.Hitbox`))))
  ;[1 1 1] Button Pushing down
  (if (`self.enabled`)
    ;[1 1 1] Calls Recording Stop
    (bind _outactors (`GameplayStatics.GetAllActorsOfClass` "/Game/Stutter_Speak_Content/Blueprints/Recording_Test.Recording_Test_C"))
    (bind _asrecording_test (cast `/Game/Stutter_Speak_Content/Blueprints/Recording_Test` (`|GetArrayItem` _outactors)))
    (`/Game/Stutter_Speak_Content/Blueprints/Recording_Test.CalledByButtonStop` _asrecording_test)
    ;[1 1 1] Calls Rater Interface
    (bind _outactors_2 (`GameplayStatics.GetAllActorsOfClass` "/Game/Stutter_Speak_Content/Widgets/BPRater.BPRater_C"))
    (bind _asbprater (cast `/Game/Stutter_Speak_Content/Widgets/BPRater` (`|GetArrayItem` _outactors_2)))
    (`self.SetActorHiddenInGame` _asbprater false)
    (`SceneComponent.SetVisibility` (`/Game/Stutter_Speak_Content/Widgets/BPRater.Widget` _asbprater) true false)
    (`SceneComponent.SetVisibility` (`/Game/Stutter_Speak_Content/Widgets/BPRater.DefaultSceneRoot` _asbprater) true false)
    (if (> _returnvalue_z _returnvalue_z_2)
      (`KismetSystemLibrary.MoveComponentTo` (`self.Button Top`) (0.0 0.0 38.0) (struct) false false 0.0)
      ;;[1 1 1] These are world events (remove for final use)
      (`AudioComponent.Play` (`self.Audio`) 0.0)
      (set `self.isPressedDown` true))))

(event `self.Hitbox.OnComponentEndOverlap`
  (params (OverlappedComponent :type "PrimitiveComponent Object Reference") (OtherActor :type "Actor Object Reference") (OtherComp :type "PrimitiveComponent Object Reference") (OtherBodyIndex :type Integer))
  ;[1 1 1] Releasing Button
  (if (`self.isPressedDown`)
    (`KismetSystemLibrary.MoveComponentTo` (`self.Button Top`) (0.0 0.0 68.0) (struct) false false 0.0)
    (set `self.isPressedDown` false)
    ;[1 1 1] Sets Speech On to false
    (bind _outactors (`GameplayStatics.GetAllActorsOfClass` "/Game/Starter_Content/VirtualRealityBP/Blueprints/MotionControllerPawn.MotionControllerPawn_C"))
    (bind _asmotion_controller_pawn (cast `/Game/Starter_Content/VirtualRealityBP/Blueprints/MotionControllerPawn` (`|GetArrayItem` _outactors)))
    (set `/Game/Starter_Content/VirtualRealityBP/Blueprints/MotionControllerPawn.SpeechOn` false _asmotion_controller_pawn)
    (`self.K2_DestroyActor`)))

(fn `UserConstructionScript`)