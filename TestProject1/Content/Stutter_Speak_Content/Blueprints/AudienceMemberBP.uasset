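; Audience member actor with a static mesh that gets its own audience texture when play begins.
; BeginPlay creates a dynamic instance of the audience material and sets its texture from an array on MenuGI, the game instance.
; A shared turn counter on MenuGI advances with each member and wraps at a hardcoded limit, so members cycle through the textures in spawn order rather than randomly.
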(event `self.ReceiveBeginPlay`
  (bind _returnvalue (`KismetMaterialLibrary.CreateDynamicMaterialInstance` "/Game/Stutter_Speak_Content/Materials/AudienceMembers/AudienceMAT.AudienceMAT"))
  (bind _output_get (set `self.Material` _returnvalue))
  (bind _asmenu_gi (cast `/Game/Stutter_Speak_Content/Blueprints/MenuGI` (`GameplayStatics.GetGameInstance`)))
  (bind _audienceturn (`/Game/Stutter_Speak_Content/Blueprints/MenuGI.AudienceTurn` _asmenu_gi))
  (if (!= _audienceturn 54) :!label _label
    (`MaterialInstanceDynamic.SetTextureParameterValue` _output_get "Audience" (`|GetArrayItem` (`/Game/Stutter_Speak_Content/Blueprints/MenuGI.AudienceMaterialsVar` _asmenu_gi) _audienceturn))
    (`PrimitiveComponent.SetMaterial` (`self.StaticMeshComponent`) 0 (`self.Material`))
    (`/Engine/EditorBlueprintResources/StandardMacros.IncrementInt` (`/Game/Stutter_Speak_Content/Blueprints/MenuGI.AudienceTurn` _asmenu_gi))
    (else
      (set `/Game/Stutter_Speak_Content/Blueprints/MenuGI.AudienceTurn` 0 _asmenu_gi)
      (goto _label))))

(fn `UserConstructionScript`)