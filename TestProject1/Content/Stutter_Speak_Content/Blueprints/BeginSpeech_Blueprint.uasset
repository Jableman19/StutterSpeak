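; A pressable 3D Begin button that starts loading a speech through MenuWorldLevelHolder's SpeechLoaderByDetailsPanel.
; It begins hidden without collision, and Tick swaps its enabled or disabled material from the Active flag.
; When active, an overlap by a "HandHit" component from above lowers the mesh, plays a lower-pitched sound and calls the loader.
; The release runs right after that call in the same chain, not on end overlap.
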(event `self.ReceiveTick`
  (params (DeltaSeconds :type "Float (single-precision)"))
  (if (`self.Active`)
    (`PrimitiveComponent.SetMaterial` (`self.StaticMeshComponent`) 0 "/Game/Stutter_Speak_Content/Materials/ButtonMaterials/Begin_Enabled.Begin_Enabled")
    (else
      (`PrimitiveComponent.SetMaterial` (`self.StaticMeshComponent`) 0 "/Game/Stutter_Speak_Content/Materials/ButtonMaterials/Begin_Disabled.Begin_Disabled"))))

(event `self.ReceiveBeginPlay`
  (`self.SetActorHiddenInGame` true)
  (`PrimitiveComponent.SetCollisionEnabled` (`self.StaticMeshComponent`) "NoCollision"))

(event `self.StaticMeshComponent.OnComponentBeginOverlap`
  (params (OverlappedComponent :type "PrimitiveComponent Object Reference") (OtherActor :type "Actor Object Reference") (OtherComp :type "PrimitiveComponent Object Reference") (OtherBodyIndex :type Integer) (bFromSweep :type Boolean) (SweepResult :type "HitResult Structure (by ref)"))
  (bind (_returnvalue_x _returnvalue_y _returnvalue_z) (`KismetMathLibrary.BreakVector` (`SceneComponent.K2_GetComponentLocation` OtherComp)))
  (bind _sound (`self.Sound`))
  (bind (_returnvalue_x_2 _returnvalue_y_2 _returnvalue_z_2) (`KismetMathLibrary.BreakVector` (`SceneComponent.K2_GetComponentLocation` (`self.StaticMeshComponent`))))
  (bind _returnvalue (`SceneComponent.GetRelativeTransform` (`self.StaticMeshComponent`)))
  (bind _returnvalue_2 (`SceneComponent.GetRelativeTransform` (`self.StaticMeshComponent`)))
  ;[1 1 1] Pressed Down
  (if (`self.Active`)
    (if (> _returnvalue_z _returnvalue_z_2)
      (if (`KismetStringLibrary.EqualEqual_StrStr` (`KismetSystemLibrary.GetObjectName` OtherComp) "HandHit")
        (if (not (`self.isPressedDown`))
          (`SceneComponent.K2_SetRelativeTransform` (`self.StaticMeshComponent`) (`KismetMathLibrary.MakeTransform` (`KismetMathLibrary.MakeVector` (.x (.location _returnvalue_2)) (.y (.location _returnvalue_2)) (- (.z (.location _returnvalue_2)) 1.0)) (.rotation _returnvalue_2) (.scale _returnvalue_2)) false false)
          (`AudioComponent.SetPitchMultiplier` _sound 0.75)
          (`AudioComponent.Play` _sound 0.0)
          (set `self.isPressedDown` true)
          (bind _outactors (`GameplayStatics.GetAllActorsOfClass` "/Game/Stutter_Speak_Content/Managers/MenuWorldLevelHolder.MenuWorldLevelHolder_C"))
          (bind _asmenu_world_level_holder (cast `/Game/Stutter_Speak_Content/Managers/MenuWorldLevelHolder` (`|GetArrayItem` _outactors)))
          (`/Game/Stutter_Speak_Content/Managers/MenuWorldLevelHolder.SpeechLoaderByDetailsPanel` _asmenu_world_level_holder)
          ;[1 1 1] Released
          (if (`self.isPressedDown`)
            (`SceneComponent.K2_SetRelativeTransform` (`self.StaticMeshComponent`) (`KismetMathLibrary.MakeTransform` (`KismetMathLibrary.MakeVector` (.x (.location _returnvalue)) (.y (.location _returnvalue)) (+ (.z (.location _returnvalue)) 1.0)) (.rotation _returnvalue) (.scale _returnvalue)) false false)
            (set `self.isPressedDown` false)))))))

(fn `UserConstructionScript`)