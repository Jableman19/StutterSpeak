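; Half-circle table actor for a VR speech scene that can be raised for post-speech actions.
; On BeginPlay it stores the static mesh's world location as the spawn location.
; Its raise event, named for Level Blueprint use, finds the first MotionControllerPawn and moves the table up by adding the pawn camera's world Z to the table's current Z, keeping X and Y.
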(event `self.ReceiveBeginPlay`
  (set `self.Spawn Location` (`SceneComponent.K2_GetComponentLocation` (`self.StaticMeshComponent`))))

(event `RaiseTableByLevelBlueprint`
  (bind (_returnvalue_x _returnvalue_y _returnvalue_z) (`KismetMathLibrary.BreakVector` (`self.K2_GetActorLocation`)))
  ;[1 1 1] Rasies Table for Post Speech Actions
  (bind _outactors (`GameplayStatics.GetAllActorsOfClass` "/Game/Starter_Content/VirtualRealityBP/Blueprints/MotionControllerPawn.MotionControllerPawn_C"))
  (bind _asmotion_controller_pawn (cast `/Game/Starter_Content/VirtualRealityBP/Blueprints/MotionControllerPawn` (`|GetArrayItem` _outactors)))
  (bind (_returnvalue_x_2 _returnvalue_y_2 _returnvalue_z_2) (`KismetMathLibrary.BreakVector` (`SceneComponent.K2_GetComponentLocation` (`/Game/Starter_Content/VirtualRealityBP/Blueprints/MotionControllerPawn.Camera` _asmotion_controller_pawn))))
  (`self.K2_SetActorLocation` (`KismetMathLibrary.MakeVector` _returnvalue_x _returnvalue_y (+ _returnvalue_z_2 _returnvalue_z))))

(fn `UserConstructionScript`)