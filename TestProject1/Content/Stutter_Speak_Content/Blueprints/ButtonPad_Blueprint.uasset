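; ButtonPad actor that responds to speech begin and cancel events, apparently for a speaking exercise.
; The begin-button event plays its audio component as a humming sound and stops it after a short delay.
; Begin-speech and cancel events find the first RightButton and LeftButton in the level and toggle their ButtonOn flags, disabling and re-enabling the arrow controls.
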(event `PlayHummingByBeginButton`
  (bind _audio (`self.Audio`))
  (`AudioComponent.Play` _audio 0.0)
  (`AudioComponent.StopDelayed` _audio 1.75))

(event `DisableArrowButtonsByBeginSpeech`
  (bind _outactors (`GameplayStatics.GetAllActorsOfClass` "/Game/Stutter_Speak_Content/Pre-Fabs/CompleteModels/RightButton.RightButton_C"))
  (bind _asright_button (cast `/Game/Stutter_Speak_Content/Pre-Fabs/CompleteModels/RightButton` (`|GetArrayItem` _outactors)))
  (set `/Game/Stutter_Speak_Content/Pre-Fabs/CompleteModels/RightButton.ButtonOn` false _asright_button)
  (bind _outactors_2 (`GameplayStatics.GetAllActorsOfClass` "/Game/Stutter_Speak_Content/Pre-Fabs/CompleteModels/LeftButton.LeftButton_C"))
  (bind _asleft_button (cast `/Game/Stutter_Speak_Content/Pre-Fabs/CompleteModels/LeftButton` (`|GetArrayItem` _outactors_2)))
  (set `/Game/Stutter_Speak_Content/Pre-Fabs/CompleteModels/LeftButton.ButtonOn` false _asleft_button))

(event `RenableArrowButtonsByCancel`
  (bind _outactors (`GameplayStatics.GetAllActorsOfClass` "/Game/Stutter_Speak_Content/Pre-Fabs/CompleteModels/RightButton.RightButton_C"))
  (bind _asright_button (cast `/Game/Stutter_Speak_Content/Pre-Fabs/CompleteModels/RightButton` (`|GetArrayItem` _outactors)))
  (set `/Game/Stutter_Speak_Content/Pre-Fabs/CompleteModels/RightButton.ButtonOn` true _asright_button)
  (bind _outactors_2 (`GameplayStatics.GetAllActorsOfClass` "/Game/Stutter_Speak_Content/Pre-Fabs/CompleteModels/LeftButton.LeftButton_C"))
  (bind _asleft_button (cast `/Game/Stutter_Speak_Content/Pre-Fabs/CompleteModels/LeftButton` (`|GetArrayItem` _outactors_2)))
  (set `/Game/Stutter_Speak_Content/Pre-Fabs/CompleteModels/LeftButton.ButtonOn` true _asleft_button))

(fn `UserConstructionScript`)