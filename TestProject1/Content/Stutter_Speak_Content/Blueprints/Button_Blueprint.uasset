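; A physical VR push button that returns the player to the MenuWorld level when released.
; Overlaps from above the hitbox lower the button top, toggle the display text and play audio.
; When the overlap ends after a press, it raises the top, toggles the text again and saves the MotionControllerPawn camera yaw to MenuGI as RotationOffset before loading the level.
; The text and audio feedback are marked as temporary.
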(event `self.Hitbox.OnComponentBeginOverlap`
  (params (OverlappedComponent :type "PrimitiveComponent Object Reference") (OtherActor :type "Actor Object Reference") (OtherComp :type "PrimitiveComponent Object Reference") (OtherBodyIndex :type Integer) (bFromSweep :type Boolean) (SweepResult :type "HitResult Structure (by ref)"))
  (bind (_returnvalue_x _returnvalue_y _returnvalue_z) (`KismetMathLibrary.BreakVector` (`SceneComponent.K2_GetComponentLocation` OtherComp)))
  (bind (_returnvalue_x_2 _returnvalue_y_2 _returnvalue_z_2) (`KismetMathLibrary.BreakVector` (`SceneComponent.K2_GetComponentLocation` (`self.Hitbox`))))
  ;[1 1 1] Button Pushing down
  (if (> _returnvalue_z _returnvalue_z_2)
    (`KismetSystemLibrary.MoveComponentTo` (`self.Button Top`) (0.0 0.0 38.0) (struct) false false 0.0)
    ;;[1 1 1] These are world events (remove for final use)
    (`SceneComponent.ToggleVisibility` (`self.Display Text`) false)
    (`AudioComponent.Play` (`self.Audio`) 0.0)
    (set `self.isPressedDown` true)))

(event `self.Hitbox.OnComponentEndOverlap`
  (params (OverlappedComponent :type "PrimitiveComponent Object Reference") (OtherActor :type "Actor Object Reference") (OtherComp :type "PrimitiveComponent Object Reference") (OtherBodyIndex :type Integer))
  ;[1 1 1] Releasing Button
  (if (`self.isPressedDown`)
    (`KismetSystemLibrary.MoveComponentTo` (`self.Button Top`) (0.0 0.0 68.0) (struct) false false 0.0)
    ;;[1 1 1] World Event (remove for final use)
    (`SceneComponent.ToggleVisibility` (`self.Display Text`) false)
    (set `self.isPressedDown` false)
    (bind _outactors (`GameplayStatics.GetAllActorsOfClass` "/Game/Starter_Content/VirtualRealityBP/Blueprints/MotionControllerPawn.MotionControllerPawn_C"))
    (bind _asmotion_controller_pawn (cast `/Game/Starter_Content/VirtualRealityBP/Blueprints/MotionControllerPawn` (`|GetArrayItem` _outactors)))
    (bind _asmenu_gi (cast `/Game/Stutter_Speak_Content/Blueprints/MenuGI` (`GameplayStatics.GetGameInstance`)))
    (bind (_returnvalue_roll _returnvalue_pitch _returnvalue_yaw) (`KismetMathLibrary.BreakRotator` (`SceneComponent.K2_GetComponentRotation` (`/Game/Starter_Content/VirtualRealityBP/Blueprints/MotionControllerPawn.Camera` _asmotion_controller_pawn))))
    (set `/Game/Stutter_Speak_Content/Blueprints/MenuGI.Rotation Offset` _returnvalue_yaw _asmenu_gi)
    (`GameplayStatics.OpenLevel` "MenuWorld")))

(fn `UserConstructionScript`)