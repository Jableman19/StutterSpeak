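; Physical Retry button actor, hidden until RaiseButton slides it up and arms it; LowerButton disarms, lowers and hides it.
; An overlap from above by a HandHit component dips the cap, plays a click sound and deactivates itself plus the Retrack and Menu_Button actors.
; After a short delay it releases, sets all three buttons to the SettingsBox material and calls SpeechByWidget on LevelHandler_Blueprint.
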(event `self.ReceiveBeginPlay`
  ;[1 1 1] Hides Button at the Start
  (`self.SetActorHiddenInGame` true))

(event `self.Retry Button.OnComponentBeginOverlap`
  (params (OverlappedComponent :type "PrimitiveComponent Object Reference") (OtherActor :type "Actor Object Reference") (OtherComp :type "PrimitiveComponent Object Reference") (OtherBodyIndex :type Integer) (bFromSweep :type Boolean) (SweepResult :type "HitResult Structure (by ref)"))
  (bind (_returnvalue_x _returnvalue_y _returnvalue_z) (`KismetMathLibrary.BreakVector` (`SceneComponent.K2_GetComponentLocation` OtherComp)))
  (bind _sound (`self.Sound`))
  (bind (_returnvalue_x_2 _returnvalue_y_2 _returnvalue_z_2) (`KismetMathLibrary.BreakVector` (`SceneComponent.K2_GetComponentLocation` (`self.Retry Button`))))
  (bind (_returnvalue_location _returnvalue_rotation _returnvalue_scale) (`KismetMathLibrary.BreakTransform` (`SceneComponent.GetRelativeTransform` (`self.Retry Button`))))
  ;[1 1 1] Conditions for Functioning
  (if (`self.Active`)
    (set `self.Active` false)
    (if (> _returnvalue_z _returnvalue_z_2)
      (if (`KismetStringLibrary.EqualEqual_StrStr` (`KismetSystemLibrary.GetObjectName` OtherComp) "HandHit")
        (if (not (`self.isPressedDown`))
          ;[1 1 1] Moves Button Top
          (bind _output_get (set `self.Up Location` _returnvalue_location))
          (set `self.Return Value Rotation` _returnvalue_rotation)
          (set `self.Return Value Scale` _returnvalue_scale)
          (`SceneComponent.K2_SetRelativeTransform` (`self.Retry Button`) (`KismetMathLibrary.MakeTransform` (- _output_get (0.0 0.0 0.5)) (`self.Return Value Rotation`) (`self.Return Value Scale`)) false false)
          (bind _outactors (`GameplayStatics.GetAllActorsOfClass` "/Game/Stutter_Speak_Content/Blueprints/Retrack.Retrack_C"))
          (bind _asretrack (cast `/Game/Stutter_Speak_Content/Blueprints/Retrack` (`|GetArrayItem` _outactors)))
          (set `/Game/Stutter_Speak_Content/Blueprints/Retrack.Active` false _asretrack)
          (bind _outactors_2 (`GameplayStatics.GetAllActorsOfClass` "/Game/Stutter_Speak_Content/Blueprints/Menu_Button.Menu_Button_C"))
          (bind _asmenu_button (cast `/Game/Stutter_Speak_Content/Blueprints/Menu_Button` (`|GetArrayItem` _outactors_2)))
          (set `/Game/Stutter_Speak_Content/Blueprints/Menu_Button.Active` false _asmenu_button)
          ;[1 1 1] Playing Audio
          (`AudioComponent.SetPitchMultiplier` _sound 0.75)
          (`AudioComponent.Play` _sound 0.0)
          (set `self.isPressedDown` true)
          ;[1 1 1] Released
          (`KismetSystemLibrary.Delay` 0.2)
          (if (`self.isPressedDown`)
            (`SceneComponent.K2_SetRelativeTransform` (`self.Retry Button`) (`KismetMathLibrary.MakeTransform` (`self.Up Location`) (`self.Return Value Rotation`) (`self.Return Value Scale`)) false false)
            (set `self.isPressedDown` false)
            (`PrimitiveComponent.SetMaterial` (`self.Retry Button`) 0 "/Game/Stutter_Speak_Content/Materials/MenuWorldMiscMaterials/SettingsBox.SettingsBox")
            (`PrimitiveComponent.SetMaterial` (`/Game/Stutter_Speak_Content/Blueprints/Retrack.Retrack Button` _asretrack) 0 "/Game/Stutter_Speak_Content/Materials/MenuWorldMiscMaterials/SettingsBox.SettingsBox")
            (`PrimitiveComponent.SetMaterial` (`/Game/Stutter_Speak_Content/Blueprints/Menu_Button.Menu Button` _asmenu_button) 0 "/Game/Stutter_Speak_Content/Materials/MenuWorldMiscMaterials/SettingsBox.SettingsBox")
            (bind _outactors_3 (`GameplayStatics.GetAllActorsOfClass` "/Game/Stutter_Speak_Content/Widgets/Speech_World/LevelHandler_Blueprint.LevelHandler_Blueprint_C"))
            (bind _aslevel_handler_blueprint (cast `/Game/Stutter_Speak_Content/Widgets/Speech_World/LevelHandler_Blueprint` (`|GetArrayItem` _outactors_3)))
            (`/Game/Stutter_Speak_Content/Widgets/Speech_World/LevelHandler_Blueprint.SpeechByWidget` _aslevel_handler_blueprint)))))))

(event `RaiseButton`
  (bind _defaultsceneroot (`self.DefaultSceneRoot`))
  ;[1 1 1] Raises Button When Called
  (`self.SetActorHiddenInGame` false)
  (`KismetSystemLibrary.MoveComponentTo` _defaultsceneroot (+ (`SceneComponent.RelativeLocation` _defaultsceneroot) (0.0 0.0 15.0)) (`SceneComponent.RelativeRotation` _defaultsceneroot) false false 1.0)
  (set `self.Active` true))

(event `Lower Button`
  (bind _defaultsceneroot (`self.DefaultSceneRoot`))
  ;[1 1 1] Lower Button When Called
  (set `self.Active` false)
  (`KismetSystemLibrary.MoveComponentTo` _defaultsceneroot (+ (`SceneComponent.RelativeLocation` _defaultsceneroot) (0.0 0.0 -15.0)) (`SceneComponent.RelativeRotation` _defaultsceneroot) false false 1.0)
  (`self.SetActorHiddenInGame` true))

(fn `UserConstructionScript`)