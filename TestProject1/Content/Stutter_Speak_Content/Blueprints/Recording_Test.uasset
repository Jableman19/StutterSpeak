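; Test Blueprint that records microphone audio to timestamped WAV files through start and stop events meant for buttons.
; Start runs the AudioCapture and begins output recording on the Record_Mic_Audio submix.
; Stop exports the recording to a subdirectory of the project, named by date and 12-hour time without AM/PM, and stops capture.
; It then stores the folder path and notifies the Playback_Actor through RecordOver.
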(event `CalledByButtonStart`
  ;[1 1 1] Starts recording from the audio capture actor to a submix
  (`SynthComponent.Start` (`self.AudioCapture`))
  (`AudioMixerBlueprintLibrary.StartRecordingOutput` 0.0 "/Game/Stutter_Speak_Content/Record_Mic_Audio.Record_Mic_Audio"))

(event `CalledByButtonStop`
  (bind _returnvalue (`KismetMathLibrary.Now`))
  (bind _returnvalue_2 (`KismetMathLibrary.GetHour` _returnvalue))
  (bind _returnvalue_3 (`KismetTextLibrary.Conv_TextToString` (`|FormatText` "{MainDir}{SubDir}" (`KismetTextLibrary.Conv_StringToText` (`KismetSystemLibrary.GetProjectDirectory`)) (`self.SubDirectory`))))
  ;[1 1 1] Stops recording from the audio capture actor to a submix
  (if (> _returnvalue_2 12)
    (set `self.12-Hour Hour` (- _returnvalue_2 12))
    (else
      (set `self.12-Hour Hour` _returnvalue_2)))
  (`AudioMixerBlueprintLibrary.StopRecordingOutput` "WavFile" (`KismetTextLibrary.Conv_TextToString` (`|FormatText` "Recording {Month}.{Day}.{Year}_{Hour}.{Min}.{Second}" (`KismetMathLibrary.GetMonth` _returnvalue) (`KismetMathLibrary.GetDay` _returnvalue) (`KismetStringLibrary.Conv_IntToString` (`KismetMathLibrary.GetYear` _returnvalue)) (`self.12-Hour Hour`) (`KismetMathLibrary.GetMinute` _returnvalue) (`KismetMathLibrary.GetSecond` _returnvalue))) _returnvalue_3 "/Game/Stutter_Speak_Content/Record_Mic_Audio.Record_Mic_Audio" null)
  (`SynthComponent.Stop` (`self.AudioCapture`))
  (set `self.filePathway` _returnvalue_3)
  (bind _outactors (`GameplayStatics.GetAllActorsOfClass` null))
  (bind _asplayback_actor (cast `/Game/Stutter_Speak_Content/Playback_Actor` (`|GetArrayItem` _outactors)))
  (`/Game/Stutter_Speak_Content/Playback_Actor.RecordOver` _asplayback_actor))

(fn `UserConstructionScript`)