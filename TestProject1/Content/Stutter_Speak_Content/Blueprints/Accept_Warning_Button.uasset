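; VR warning-screen button that the player presses by hand to accept and continue to the MenuWorld level.
; On start it places itself below the pawn's camera height and plays a timeline intended to fade the pawn's Fader material.
; A HandHit overlap from above briefly depresses the button with sound, then reverses the timeline.
; After a delay it saves camera yaw to MenuGI as a rotation offset and opens MenuWorld.
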(event `self.ReceiveBeginPlay`
  (bind (_returnvalue_x _returnvalue_y) (`KismetMathLibrary.BreakVector` (`self.K2_GetActorLocation`)))
  ;[1 1 1] Sets Correct Height
  (`KismetSystemLibrary.Delay` 0.2)
  (bind _outactors (`GameplayStatics.GetAllActorsOfClass` "/Game/Starter_Content/VirtualRealityBP/Blueprints/MotionControllerPawn.MotionControllerPawn_C"))
  (bind _asmotion_controller_pawn (cast `/Game/Starter_Content/VirtualRealityBP/Blueprints/MotionControllerPawn` (`|GetArrayItem` _outactors)))
  (bind (_returnvalue_x_2 _returnvalue_y_2 _returnvalue_z) (`KismetMathLibrary.BreakVector` (`SceneComponent.K2_GetComponentLocation` (`/Game/Starter_Content/VirtualRealityBP/Blueprints/MotionControllerPawn.Camera` _asmotion_controller_pawn))))
  (`self.K2_SetActorLocation` (`KismetMathLibrary.MakeVector` _returnvalue_x _returnvalue_y (- _returnvalue_z 60.0)))
  ;[1 1 1] Hides Fader
  (bind _returnvalue (`KismetMaterialLibrary.CreateDynamicMaterialInstance` "/Game/Stutter_Speak_Content/Materials/FaderMaterial.FaderMaterial"))
  (bind _output_get (set `self.MAT` _returnvalue))
  (`PrimitiveComponent.SetMaterial` (`/Game/Starter_Content/VirtualRealityBP/Blueprints/MotionControllerPawn.Fader` _asmotion_controller_pawn) 0 _output_get)
  (`TimelineComponent.Play` (`self.Timeline_0`)))

(event `self.Confirm Button.OnComponentBeginOverlap`
  (params (OverlappedComponent :type "PrimitiveComponent Object Reference") (OtherActor :type "Actor Object Reference") (OtherComp :type "PrimitiveComponent Object Reference") (OtherBodyIndex :type Integer) (bFromSweep :type Boolean) (SweepResult :type "HitResult Structure (by ref)"))
  (bind (_returnvalue_x _returnvalue_y _returnvalue_z) (`KismetMathLibrary.BreakVector` (`SceneComponent.K2_GetComponentLocation` OtherComp)))
  (bind _sound (`self.Sound`))
  (bind (_returnvalue_x_2 _returnvalue_y_2 _returnvalue_z_2) (`KismetMathLibrary.BreakVector` (`SceneComponent.K2_GetComponentLocation` (`self.Confirm Button`))))
  (bind (_returnvalue_location _returnvalue_rotation _returnvalue_scale) (`KismetMathLibrary.BreakTransform` (`SceneComponent.GetRelativeTransform` (`self.Confirm Button`))))
  ;[1 1 1] Conditions for Functioning
  (if (`self.Active`)
    (if (> _returnvalue_z _returnvalue_z_2)
      (if (`KismetStringLibrary.EqualEqual_StrStr` (`KismetSystemLibrary.GetObjectName` OtherComp) "HandHit")
        (if (not (`self.isPressedDown`))
          ;[1 1 1] Moves Button Top
          (bind _output_get (set `self.Up Location` _returnvalue_location))
          (set `self.Return Value Rotation` _returnvalue_rotation)
          (set `self.Return Value Scale` _returnvalue_scale)
          (`SceneComponent.K2_SetRelativeTransform` (`self.Confirm Button`) (`KismetMathLibrary.MakeTransform` (- _output_get (0.0 0.0 0.5)) (`self.Return Value Rotation`) (`self.Return Value Scale`)) false false)
          ;[1 1 1] Playing Audio
          (`AudioComponent.SetPitchMultiplier` _sound 0.75)
          (`AudioComponent.Play` _sound 0.0)
          (set `self.isPressedDown` true)
          ;[1 1 1] Released
          (`KismetSystemLibrary.Delay` 0.2)
          (if (`self.isPressedDown`)
            (`SceneComponent.K2_SetRelativeTransform` (`self.Confirm Button`) (`KismetMathLibrary.MakeTransform` (`self.Up Location`) (`self.Return Value Rotation`) (`self.Return Value Scale`)) false false)
            ;[1 1 1] Unhides Fader and Opens New Level
            (`TimelineComponent.Reverse` (`self.Timeline_0`))
            (`KismetSystemLibrary.Delay` 2.5)
            (bind _asmenu_gi (cast `/Game/Stutter_Speak_Content/Blueprints/MenuGI` (`GameplayStatics.GetGameInstance`)))
            (bind (_returnvalue_roll _returnvalue_pitch _returnvalue_yaw) (`KismetMathLibrary.BreakRotator` (`SceneComponent.K2_GetComponentRotation` (`/Game/Starter_Content/VirtualRealityBP/Blueprints/MotionControllerPawn.Camera` (stale `self.ReceiveBeginPlay` _asmotion_controller_pawn)))))
            (set `/Game/Stutter_Speak_Content/Blueprints/MenuGI.Rotation Offset` _returnvalue_yaw _asmenu_gi)
            (`GameplayStatics.OpenLevel` "MenuWorld")))))))

(fn `UserConstructionScript`)