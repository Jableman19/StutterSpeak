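; Clickable in-world slider for choosing Small, Medium or Large text size, with an LED for each setting.
; On BeginPlay it reads TextSize from MenuGI to set the slider position and LEDs, then finds the SettingsBox.
; Each Pickup steps a four-state index that ping-pongs through the sizes, with Medium appearing in both directions.
; Each step moves the slider, swaps LED materials, plays audio and calls the matching SettingsBox switch.
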(event `self.ReceiveBeginPlay`
  ;[1 1 1] Sets correct color and location on spawn
  (bind _asmenu_gi (cast `/Game/Stutter_Speak_Content/Blueprints/MenuGI` (`GameplayStatics.GetGameInstance`)))
  (bind _textsize (`/Game/Stutter_Speak_Content/Blueprints/MenuGI.TextSize` _asmenu_gi))
  (if (`KismetStringLibrary.EqualEqual_StrStr` _textsize "Small")
    (set `self.New location` (0.0 10.0 0.0))
    (`self.Reset LEDS` (`self.LED (Small)`) (`self.LED (Meduim)`) (`self.LED (Large)`))
    (set `self.Current Index` 0)
    (elif (`KismetStringLibrary.EqualEqual_StrStr` _textsize "Medium")
      (set `self.New location` (0.0 0.0 0.0))
      (`self.Reset LEDS` (`self.LED (Meduim)`) (`self.LED (Large)`) (`self.LED (Small)`))
      (set `self.Current Index` 1)
      (else
        (set `self.New location` (0.0 -10.0 0.0))
        (`self.Reset LEDS` (`self.LED (Large)`) (`self.LED (Small)`) (`self.LED (Meduim)`))
        (set `self.Current Index` 2))))
  (`SceneComponent.K2_SetRelativeLocation` (`self.Slider`) (`self.New location`) false false)
  (bind _returnvalue (`GameplayStatics.GetActorOfClass` "/Game/Stutter_Speak_Content/Blueprints/SettingsBox.SettingsBox_C"))
  (bind _assettings_box (cast `/Game/Stutter_Speak_Content/Blueprints/SettingsBox` _returnvalue))
  (set `self.As Settings Box` _assettings_box))

(event `/Game/Starter_Content/VirtualRealityBP/Blueprints/PickupActorInterface.Pickup`
  (params (AttachTo :type "SceneComponent Object Reference"))
  ;[1 1 1] Updating Slider on Click
  (switch `int` (`self.Current Index`)
    (:`0`
      (set `self.Next Index` 1))
    (:`1`
      (set `self.Next Index` 2))
    (:`2`
      (set `self.Next Index` 3))
    (:`3`
      (set `self.Next Index` 0)))
  (switch `int` (`self.Next Index`)
    (:`0`
      (`self.Change LEDS` (`self.LED (Small)`) (`self.LED (Meduim)`))
      (set `self.New location` (0.0 10.0 0.0))
      (set `self.Current Index` 0)
      (`/Game/Stutter_Speak_Content/Blueprints/SettingsBox.SmallBySmallSwitch` (`self.As Settings Box`)))
    (:`1`
      (`self.Change LEDS` (`self.LED (Meduim)`) (`self.LED (Small)`))
      (set `self.New location` (0.0 0.0 0.0))
      (set `self.Current Index` 1)
      (`/Game/Stutter_Speak_Content/Blueprints/SettingsBox.MediumByMediumSwitch` (`self.As Settings Box`)))
    (:`2`
      (`self.Change LEDS` (`self.LED (Large)`) (`self.LED (Meduim)`))
      (set `self.New location` (0.0 -10.0 0.0))
      (set `self.Current Index` 2)
      (`/Game/Stutter_Speak_Content/Blueprints/SettingsBox.LargeByLargeSwitch` (`self.As Settings Box`)))
    (:`3`
      (`self.Change LEDS` (`self.LED (Meduim)`) (`self.LED (Large)`))
      (set `self.New location` (0.0 0.0 0.0))
      (set `self.Current Index` 3)
      (`/Game/Stutter_Speak_Content/Blueprints/SettingsBox.MediumByMediumSwitch` (`self.As Settings Box`))))
  (`AudioComponent.Play` (`self.Audio`) 0.0)
  (`SceneComponent.K2_SetRelativeLocation` (`self.Slider`) (`self.New location`) false false))

(fn `Change LEDS`
  (params (`LED On` :type "StaticMeshComponent Object Reference") (`LED Off` :type "StaticMeshComponent Object Reference"))
  (`PrimitiveComponent.SetMaterial` `LED On` 0 "/Game/Stutter_Speak_Content/Materials/MenuWorldMiscMaterials/LED_On.LED_On")
  (`PrimitiveComponent.SetMaterial` `LED Off` 0 "/Game/Stutter_Speak_Content/Materials/MenuWorldMiscMaterials/LED_Off.LED_Off"))

(fn `Reset LEDS`
  (params (`LED On` :type "StaticMeshComponent Object Reference") (`LED Off (1)` :type "StaticMeshComponent Object Reference") (`LED Off (2)` :type "StaticMeshComponent Object Reference"))
  (`PrimitiveComponent.SetMaterial` `LED On` 0 "/Game/Stutter_Speak_Content/Materials/MenuWorldMiscMaterials/LED_On.LED_On")
  (`PrimitiveComponent.SetMaterial` `LED Off (1)` 0 "/Game/Stutter_Speak_Content/Materials/MenuWorldMiscMaterials/LED_Off.LED_Off")
  (`PrimitiveComponent.SetMaterial` `LED Off (2)` 0 "/Game/Stutter_Speak_Content/Materials/MenuWorldMiscMaterials/LED_Off.LED_Off"))

(fn `UserConstructionScript`)