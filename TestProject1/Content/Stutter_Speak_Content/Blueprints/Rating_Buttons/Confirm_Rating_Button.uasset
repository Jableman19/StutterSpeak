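; Confirm button for the post-speech self-rating step, pressed from above by an overlapping HandHit component while Active.
; A press lowers the button, plays a click and, if a rating is selected, writes it to MenuGI.
; A FirstTime flag alternates two stages: message satisfaction advances the projector screen widget, then fluency satisfaction triggers saving and displays results.
; The button rises only within those stages, so a press without a selection leaves it down.
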(event `self.Confirm Button.OnComponentBeginOverlap`
  (params (OverlappedComponent :type "PrimitiveComponent Object Reference") (OtherActor :type "Actor Object Reference") (OtherComp :type "PrimitiveComponent Object Reference") (OtherBodyIndex :type Integer) (bFromSweep :type Boolean) (SweepResult :type "HitResult Structure (by ref)"))
  (bind (_returnvalue_x _returnvalue_y _returnvalue_z) (`KismetMathLibrary.BreakVector` (`SceneComponent.K2_GetComponentLocation` OtherComp)))
  (bind _selected_rating (`self.Selected Rating`))
  (bind _sound (`self.Sound`))
  (bind _as_hanging_projector_screen_blueprint (`self.As Hanging Projector Screen Blueprint`))
  (bind (_returnvalue_x_2 _returnvalue_y_2 _returnvalue_z_2) (`KismetMathLibrary.BreakVector` (`SceneComponent.K2_GetComponentLocation` (`self.Confirm Button`))))
  (bind _returnvalue (`SceneComponent.GetRelativeTransform` (`self.Confirm Button`)))
  (bind _returnvalue_2 (`SceneComponent.GetRelativeTransform` (`self.Confirm Button`)))
  (bind _returnvalue_3 (`SceneComponent.GetRelativeTransform` (`self.Confirm Button`)))
  ;[1 1 1] Pressed Down
  (if (`self.Active`)
    (if (> _returnvalue_z _returnvalue_z_2)
      (if (`KismetStringLibrary.EqualEqual_StrStr` (`KismetSystemLibrary.GetObjectName` OtherComp) "HandHit")
        (if (not (`self.isPressedDown`))
          (`SceneComponent.K2_SetRelativeTransform` (`self.Confirm Button`) (`KismetMathLibrary.MakeTransform` (`KismetMathLibrary.MakeVector` (.x (.location _returnvalue_3)) (.y (.location _returnvalue_3)) (- (.z (.location _returnvalue_3)) 1.0)) (.rotation _returnvalue_3) (.scale _returnvalue_3)) false false)
          (`AudioComponent.SetPitchMultiplier` _sound 0.75)
          (`AudioComponent.Play` _sound 0.0)
          (set `self.isPressedDown` true)
          (if (!= (`self.Selected Rating`) 0)
            (bind _outactors (`GameplayStatics.GetAllActorsOfClass` "/Game/Stutter_Speak_Content/Blueprints/Hanging_Projector_Screen_Blueprint.Hanging_Projector_Screen_Blueprint_C"))
            (bind _ashanging_projector_screen_blueprint (cast `/Game/Stutter_Speak_Content/Blueprints/Hanging_Projector_Screen_Blueprint` (`|GetArrayItem` _outactors)))
            (bind _output_get (set `self.As Hanging Projector Screen Blueprint` _ashanging_projector_screen_blueprint))
            (bind _asmenu_gi (cast `/Game/Stutter_Speak_Content/Blueprints/MenuGI` (`GameplayStatics.GetGameInstance`)))
            (if (`self.First Time`)
              ;[1 1 1] Sets User Rating in the Struct
              (set `/Game/Stutter_Speak_Content/Blueprints/MenuGI.Data to Save : Message Satisfacation Rating` _selected_rating _asmenu_gi)
              ;[1 1 1] Calls Next Rating
              (`/Game/Stutter_Speak_Content/Blueprints/Hanging_Projector_Screen_Blueprint.ChangeWidget` _output_get)
              (set `self.First Time` false)
              ;[1 1 1] Released
              (if (`self.isPressedDown`)
                (`SceneComponent.K2_SetRelativeTransform` (`self.Confirm Button`) (`KismetMathLibrary.MakeTransform` (`KismetMathLibrary.MakeVector` (.x (.location _returnvalue)) (.y (.location _returnvalue)) (+ (.z (.location _returnvalue)) 1.0)) (.rotation _returnvalue) (.scale _returnvalue)) false false)
                (set `self.isPressedDown` false))
              (else
                (set `/Game/Stutter_Speak_Content/Blueprints/MenuGI.Data to Save : Fluency Satisfaction Rating` _selected_rating _asmenu_gi)
                (set `self.First Time` true)
                ;[1 1 1] Calls to Save Data
                (bind _asmenu_gi_2 (cast `/Game/Stutter_Speak_Content/Blueprints/MenuGI` (`GameplayStatics.GetGameInstance`)))
                (`/Game/Stutter_Speak_Content/Blueprints/MenuGI.Call Saving Data` _asmenu_gi_2)
                ;[1 1 1] Released
                (if (`self.isPressedDown`)
                  (`SceneComponent.K2_SetRelativeTransform` (`self.Confirm Button`) (`KismetMathLibrary.MakeTransform` (`KismetMathLibrary.MakeVector` (.x (.location _returnvalue_2)) (.y (.location _returnvalue_2)) (+ (.z (.location _returnvalue_2)) 1.0)) (.rotation _returnvalue_2) (.scale _returnvalue_2)) false false)
                  (set `self.isPressedDown` false)
                  ;[1 1 1] Makes results appear
                  (`/Game/Stutter_Speak_Content/Widgets/Speech_World/ResultsDataBP.ResultsCallbyConfirmRatingButton` (`/Game/Stutter_Speak_Content/Blueprints/Hanging_Projector_Screen_Blueprint.Results Data` _as_hanging_projector_screen_blueprint))
                  (`/Game/Stutter_Speak_Content/Blueprints/Hanging_Projector_Screen_Blueprint.DisplayResults` _as_hanging_projector_screen_blueprint))))))))))

(fn `UserConstructionScript`)