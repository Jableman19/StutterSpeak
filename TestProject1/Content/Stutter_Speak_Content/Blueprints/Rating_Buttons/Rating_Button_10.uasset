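; Rating_Button_10 is a physical push button, touched by a hand, that selects a rating of 10.
; When active, an overlap from above by the HandHit component nudges the top down, plays a lower-pitched click sound, then immediately raises it again.
; The press sets SelectedRating on the Confirm_Rating_Button and moves the Active_Choice_Ring onto this button's base.
; LowerButton disables collision, sinks the button over a second, then hides it.
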(event `self.Button Top.OnComponentBeginOverlap`
  (params (OverlappedComponent :type "PrimitiveComponent Object Reference") (OtherActor :type "Actor Object Reference") (OtherComp :type "PrimitiveComponent Object Reference") (OtherBodyIndex :type Integer) (bFromSweep :type Boolean) (SweepResult :type "HitResult Structure (by ref)"))
  (bind (_returnvalue_x _returnvalue_y _returnvalue_z) (`KismetMathLibrary.BreakVector` (`SceneComponent.K2_GetComponentLocation` OtherComp)))
  (bind _sound (`self.Sound`))
  (bind _button_base (`self.Button Base`))
  (bind (_returnvalue_x_2 _returnvalue_y_2 _returnvalue_z_2) (`KismetMathLibrary.BreakVector` (`SceneComponent.K2_GetComponentLocation` (`self.Button Top`))))
  (bind _returnvalue (`SceneComponent.GetRelativeTransform` (`self.Button Top`)))
  (bind _returnvalue_2 (`SceneComponent.GetRelativeTransform` (`self.Button Top`)))
  ;[1 1 1] Pressed Down
  (if (`self.Active`)
    (if (> _returnvalue_z _returnvalue_z_2)
      (if (`KismetStringLibrary.EqualEqual_StrStr` (`KismetSystemLibrary.GetObjectName` OtherComp) "HandHit")
        (if (not (`self.isPressedDown`))
          (`SceneComponent.K2_SetRelativeTransform` (`self.Button Top`) (`KismetMathLibrary.MakeTransform` (`KismetMathLibrary.MakeVector` (.x (.location _returnvalue_2)) (.y (.location _returnvalue_2)) (- (.z (.location _returnvalue_2)) 1.0)) (.rotation _returnvalue_2) (.scale _returnvalue_2)) false false)
          (`AudioComponent.SetPitchMultiplier` _sound 0.75)
          (`AudioComponent.Play` _sound 0.0)
          (set `self.isPressedDown` true)
          ;[1 1 1] Updates Rating and Moves Ring
          (bind _outactors (`GameplayStatics.GetAllActorsOfClass` "/Game/Stutter_Speak_Content/Blueprints/Rating_Buttons/Confirm_Rating_Button.Confirm_Rating_Button_C"))
          (bind _asconfirm_rating_button (cast `/Game/Stutter_Speak_Content/Blueprints/Rating_Buttons/Confirm_Rating_Button` (`|GetArrayItem` _outactors)))
          (set `/Game/Stutter_Speak_Content/Blueprints/Rating_Buttons/Confirm_Rating_Button.Selected Rating` 10 _asconfirm_rating_button)
          (bind _outactors_2 (`GameplayStatics.GetAllActorsOfClass` "/Game/Stutter_Speak_Content/Blueprints/Rating_Buttons/Active_Choice_Ring.Active_Choice_Ring_C"))
          (bind _asactive_choice_ring (cast `/Game/Stutter_Speak_Content/Blueprints/Rating_Buttons/Active_Choice_Ring` (`|GetArrayItem` _outactors_2)))
          (`self.K2_SetActorLocationAndRotation` _asactive_choice_ring (`SceneComponent.K2_GetComponentLocation` _button_base) (`SceneComponent.K2_GetComponentRotation` _button_base) false false)
          ;[1 1 1] Released
          (if (`self.isPressedDown`)
            (`SceneComponent.K2_SetRelativeTransform` (`self.Button Top`) (`KismetMathLibrary.MakeTransform` (`KismetMathLibrary.MakeVector` (.x (.location _returnvalue)) (.y (.location _returnvalue)) (+ (.z (.location _returnvalue)) 1.0)) (.rotation _returnvalue) (.scale _returnvalue)) false false)
            (set `self.isPressedDown` false)))))))

(event `LowerButton`
  (bind _defaultsceneroot (`self.DefaultSceneRoot`))
  (`self.SetActorEnableCollision` false)
  (`KismetSystemLibrary.MoveComponentTo` _defaultsceneroot (- (`SceneComponent.RelativeLocation` _defaultsceneroot) (0.0 0.0 15.0)) (`SceneComponent.RelativeRotation` _defaultsceneroot) false false 1.0)
  (`self.SetActorHiddenInGame` true))

(fn `UserConstructionScript`)