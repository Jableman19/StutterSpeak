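; Cancel button actor, pressed by a hand in the world, that backs out of what the Begin button started.
; It starts hidden and lowered; CancelByBegin reveals it, raises it and enables collision.
; A HandHit overlap from above plays a press bounce and sound, then notifies the button pad, checkmark, Begin button, projector and screen through GetAllActorsOfClass lookups.
; It then sinks and hides again.
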(event `CancelByBegin`
  (bind (_returnvalue_location _returnvalue_rotation) (`KismetMathLibrary.BreakTransform` (`SceneComponent.GetRelativeTransform` (`self.StaticMeshComponent`))))
  ;[1 1 1] Cancel Button Raised When Begin is Hit
  (`self.SetActorHiddenInGame` false)
  (`KismetSystemLibrary.MoveComponentTo` (`self.StaticMeshComponent`) (`self.UpLocation`) _returnvalue_rotation false false 1.0)
  (set `self.ButtonOn` true)
  (`PrimitiveComponent.SetCollisionEnabled` (`self.StaticMeshComponent`) "QueryAndPhysics"))

(event `self.ReceiveBeginPlay`
  (bind _returnvalue (`SceneComponent.GetRelativeTransform` (`self.StaticMeshComponent`)))
  (bind (_returnvalue_location _returnvalue_rotation _returnvalue_scale) (`KismetMathLibrary.BreakTransform` (`SceneComponent.GetRelativeTransform` (`self.StaticMeshComponent`))))
  ;[1 1 1] On Spawn Decides and sets values for movement
  (`self.SetActorHiddenInGame` true)
  (`PrimitiveComponent.SetCollisionEnabled` (`self.StaticMeshComponent`) "NoCollision")
  (`KismetSystemLibrary.Delay` 1.0)
  (set `self.UpLocation` (`KismetMathLibrary.MakeVector` (.x (.location _returnvalue)) (.y (.location _returnvalue)) (.z (.location _returnvalue))))
  (bind _output_get (set `self.DownLocation` (`KismetMathLibrary.MakeVector` (.x (.location _returnvalue)) (.y (.location _returnvalue)) (- (.z (.location _returnvalue)) 5.0))))
  (set `self.DownLocationSmall` (`KismetMathLibrary.MakeVector` (.x (.location _returnvalue)) (.y (.location _returnvalue)) (- (.z (.location _returnvalue)) 0.5)))
  (`SceneComponent.K2_SetRelativeTransform` (`self.StaticMeshComponent`) (`KismetMathLibrary.MakeTransform` _output_get _returnvalue_rotation _returnvalue_scale) false false))

(event `self.StaticMeshComponent.OnComponentBeginOverlap`
  (params (OverlappedComponent :type "PrimitiveComponent Object Reference") (OtherActor :type "Actor Object Reference") (OtherComp :type "PrimitiveComponent Object Reference") (OtherBodyIndex :type Integer) (bFromSweep :type Boolean) (SweepResult :type "HitResult Structure (by ref)"))
  (bind (_returnvalue_x _returnvalue_y _returnvalue_z) (`KismetMathLibrary.BreakVector` (`SceneComponent.K2_GetComponentLocation` OtherComp)))
  (bind _sound (`self.Sound`))
  (bind _staticmeshcomponent (`self.StaticMeshComponent`))
  (bind (_returnvalue_x_2 _returnvalue_y_2 _returnvalue_z_2) (`KismetMathLibrary.BreakVector` (`SceneComponent.K2_GetComponentLocation` (`self.StaticMeshComponent`))))
  (bind (_returnvalue_location _returnvalue_rotation _returnvalue_scale) (`KismetMathLibrary.BreakTransform` (`SceneComponent.GetRelativeTransform` _staticmeshcomponent)))
  (bind (_returnvalue_location_2 _returnvalue_rotation_2) (`KismetMathLibrary.BreakTransform` (`SceneComponent.GetRelativeTransform` (`self.StaticMeshComponent`))))
  ;[1 1 1] Pressed Down - Various Calls
  (if (`self.ButtonOn`)
    (if (> _returnvalue_z _returnvalue_z_2)
      (if (`KismetStringLibrary.EqualEqual_StrStr` (`KismetSystemLibrary.GetObjectName` OtherComp) "HandHit")
        (if (not (`self.isPressedDown`))
          (set `self.isPressedDown` true)
          (bind _outactors (`GameplayStatics.GetAllActorsOfClass` "/Game/Stutter_Speak_Content/Blueprints/CheckMark_BP.CheckMark_BP_C"))
          (bind _ascheck_mark_bp (cast `/Game/Stutter_Speak_Content/Blueprints/CheckMark_BP` (`|GetArrayItem` _outactors)))
          (set `/Game/Stutter_Speak_Content/Blueprints/CheckMark_BP.ButtonOn` false _ascheck_mark_bp)
          (`SceneComponent.K2_SetRelativeTransform` _staticmeshcomponent (`KismetMathLibrary.MakeTransform` (`self.DownLocationSmall`) _returnvalue_rotation _returnvalue_scale) false false)
          (`KismetSystemLibrary.Delay` 0.2)
          (`SceneComponent.K2_SetRelativeTransform` _staticmeshcomponent (`KismetMathLibrary.MakeTransform` (`self.UpLocation`) _returnvalue_rotation _returnvalue_scale) false false)
          (`AudioComponent.SetPitchMultiplier` _sound 0.75)
          (`AudioComponent.Play` _sound 0.0)
          (`KismetSystemLibrary.Delay` 0.2)
          (bind _outactors_2 (`GameplayStatics.GetAllActorsOfClass` "/Game/Stutter_Speak_Content/Blueprints/ButtonPad_Blueprint.ButtonPad_Blueprint_C"))
          (bind _asbutton_pad_blueprint (cast `/Game/Stutter_Speak_Content/Blueprints/ButtonPad_Blueprint` (`|GetArrayItem` _outactors_2)))
          (`/Game/Stutter_Speak_Content/Blueprints/ButtonPad_Blueprint.PlayHummingByBeginButton` _asbutton_pad_blueprint)
          (`KismetSystemLibrary.Delay` 0.3)
          (`/Game/Stutter_Speak_Content/Blueprints/CheckMark_BP.ConfirmByCancel` _ascheck_mark_bp)
          (`KismetSystemLibrary.MoveComponentTo` (`self.StaticMeshComponent`) (`self.DownLocation`) _returnvalue_rotation_2 false false 0.75)
          (bind _outactors_3 (`GameplayStatics.GetAllActorsOfClass` "/Game/Stutter_Speak_Content/Pre-Fabs/CompleteModels/BeginButton.BeginButton_C"))
          (bind _asbegin_button (cast `/Game/Stutter_Speak_Content/Pre-Fabs/CompleteModels/BeginButton` (`|GetArrayItem` _outactors_3)))
          (`/Game/Stutter_Speak_Content/Pre-Fabs/CompleteModels/BeginButton.BeginByCancel` _asbegin_button)
          (bind _outactors_4 (`GameplayStatics.GetAllActorsOfClass` "/Game/Stutter_Speak_Content/Blueprints/Projector_Blueprint.Projector_Blueprint_C"))
          (bind _asprojector_blueprint (cast `/Game/Stutter_Speak_Content/Blueprints/Projector_Blueprint` (`|GetArrayItem` _outactors_4)))
          (set `PrimitiveComponent.bGenerateOverlapEvents` true (`/Game/Stutter_Speak_Content/Blueprints/Projector_Blueprint.GrabBox` _asprojector_blueprint))
          (bind _outactors_5 (`GameplayStatics.GetAllActorsOfClass` "/Game/Stutter_Speak_Content/Blueprints/ProjectorScreen_Blueprint.ProjectorScreen_Blueprint_C"))
          (bind _asprojector_screen_blueprint (cast `/Game/Stutter_Speak_Content/Blueprints/ProjectorScreen_Blueprint` (`|GetArrayItem` _outactors_5)))
          (`/Game/Stutter_Speak_Content/Blueprints/ProjectorScreen_Blueprint.RevertByCancel` _asprojector_screen_blueprint)
          (`self.SetActorHiddenInGame` true)
          (`PrimitiveComponent.SetCollisionEnabled` (`self.StaticMeshComponent`) "NoCollision")
          (set `self.isPressedDown` false))))))

(fn `UserConstructionScript`)