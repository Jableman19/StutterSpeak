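; A pressable world button that writes hard-coded test save data for two speeches, Grandfather Passage and Dream Passage, despite "Load" in its name.
; An overlap from above the hitbox snaps the top down, toggles text and plays audio; ending the overlap raises it.
; Both the press and BeginPlay create a fresh SaveData object, append sample records to AllSavedData and async-save it to the "Theoretically" slot.
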(event `self.Hitbox.OnComponentBeginOverlap`
  (params (OverlappedComponent :type "PrimitiveComponent Object Reference") (OtherActor :type "Actor Object Reference") (OtherComp :type "PrimitiveComponent Object Reference") (OtherBodyIndex :type Integer) (bFromSweep :type Boolean) (SweepResult :type "HitResult Structure (by ref)"))
  (bind (_returnvalue_x _returnvalue_y _returnvalue_z) (`KismetMathLibrary.BreakVector` (`SceneComponent.K2_GetComponentLocation` OtherComp)))
  (bind (_returnvalue_x_2 _returnvalue_y_2 _returnvalue_z_2) (`KismetMathLibrary.BreakVector` (`SceneComponent.K2_GetComponentLocation` (`self.Hitbox`))))
  ;[1 1 1] Button Pushing down
  (if (> _returnvalue_z _returnvalue_z_2)
    (`KismetSystemLibrary.MoveComponentTo` (`self.Button Top`) (0.0 0.0 38.0) (struct) false false 0.0)
    ;;[1 1 1] These are world events (remove for final use)
    (`SceneComponent.ToggleVisibility` (`self.Display Text`) false)
    (`AudioComponent.Play` (`self.Audio`) 0.0)
    (set `self.isPressedDown` true)
    (bind _returnvalue (`GameplayStatics.CreateSaveGameObject` "/Game/Stutter_Speak_Content/SaveData/SaveData.SaveData_C" :!label _label))
    (bind _output_get (set `self.Data to Load` _returnvalue))
    (bind _all_saved_data (`/Game/Stutter_Speak_Content/SaveData/SaveData.All_Saved_Data` _output_get))
    (bind (_output_speechname _output_saveddataforspeechname) (break `/Game/Stutter_Speak_Content/Structs/Data_For_Each_Speech_Struct` (`|GetArrayItem` _all_saved_data)))
    (`KismetArrayLibrary.Array_Add` _output_saveddataforspeechname (make `/Game/Stutter_Speak_Content/Structs/Attempt_Struct` "Grandfather Passage" 1 626.0 602.0 30 8 7))
    (`KismetArrayLibrary.Array_Add` _output_saveddataforspeechname (make `/Game/Stutter_Speak_Content/Structs/Attempt_Struct` "Grandfather Passage" 2 900.0 712.0 86 4 5))
    (`KismetArrayLibrary.Array_Add` _output_saveddataforspeechname (make `/Game/Stutter_Speak_Content/Structs/Attempt_Struct` "Grandfather Passage" 3 1050.0 895.0 12 9 2))
    (`KismetArrayLibrary.Array_Add` _output_saveddataforspeechname (make `/Game/Stutter_Speak_Content/Structs/Attempt_Struct` "Grandfather Passage" 4 654.0 498.0 3 3 10))
    (bind (_output_speechname_2 _output_saveddataforspeechname_2) (break `/Game/Stutter_Speak_Content/Structs/Data_For_Each_Speech_Struct` (`|GetArrayItem` _all_saved_data 1)))
    (`KismetArrayLibrary.Array_Add` _output_saveddataforspeechname_2 (make `/Game/Stutter_Speak_Content/Structs/Attempt_Struct` "Dream Passage" 1 626.0 602.0 30 8 7))
    (`KismetArrayLibrary.Array_Add` _output_saveddataforspeechname_2 (make `/Game/Stutter_Speak_Content/Structs/Attempt_Struct` "Dream Passage" 2 900.0 712.0 86 4 5))
    (`KismetArrayLibrary.Array_Add` _output_saveddataforspeechname_2 (make `/Game/Stutter_Speak_Content/Structs/Attempt_Struct` "Dream Passage" 3 1050.0 895.0 12 9 2))
    (`KismetArrayLibrary.Array_Add` _output_saveddataforspeechname_2 (make `/Game/Stutter_Speak_Content/Structs/Attempt_Struct` "Dream Passage" 4 654.0 498.0 3 3 10))
    (`AsyncActionHandleSaveGame.AsyncSaveGameToSlot` (`self.Data to Load`) "Theoretically")))

(event `self.ReceiveBeginPlay`
  (goto _label))

(event `self.Hitbox.OnComponentEndOverlap`
  (params (OverlappedComponent :type "PrimitiveComponent Object Reference") (OtherActor :type "Actor Object Reference") (OtherComp :type "PrimitiveComponent Object Reference") (OtherBodyIndex :type Integer))
  ;[1 1 1] Releasing Button
  (if (`self.isPressedDown`)
    (`KismetSystemLibrary.MoveComponentTo` (`self.Button Top`) (0.0 0.0 68.0) (struct) false false 0.0)
    ;;[1 1 1] World Event (remove for final use)
    (`SceneComponent.ToggleVisibility` (`self.Display Text`) false)
    (set `self.isPressedDown` false)))

(fn `UserConstructionScript`)