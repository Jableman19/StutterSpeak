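; VR pause/play button that a hand presses from above to control playback of the player's recorded speech in a stutter retracking exercise.
; Overlaps trigger a press animation and click, swap the two shapes, and toggle playback and motion controller retracking, with Active flags gating input.
; When audio finishes, it stops the stutter timer, saves total stuttering time and displays results on the projector screen.
; External events raise, lower, reset or force-stop it.
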(event `self.ReceiveBeginPlay`
  ;[1 1 1] Resets to Default when Sequence Finishes
  (`self.SetActorHiddenInGame` true :!label _label)
  (`SceneComponent.SetVisibility` (`self.Pause_Shape`) false false)
  (`SceneComponent.SetVisibility` (`self.Play Button`) true false)
  (`PrimitiveComponent.SetMaterial` (`self.Play Button`) 0 "/Game/Starter_Content/VirtualReality/Materials/M_BaseMaterial.M_BaseMaterial")
  (`PrimitiveComponent.SetMaterial` (`self.Pause_Shape`) 0 "/Game/Starter_Content/VirtualReality/Materials/M_BaseMaterial.M_BaseMaterial")
  (`PrimitiveComponent.SetMaterial` (`self.Pause_Shape`) 1 "/Game/Starter_Content/VirtualReality/Materials/M_BaseMaterial.M_BaseMaterial")
  (set `self.First Time Start` true)
  (set `self.Complete Flag` true))

(event `Reset`
  (`SceneComponent.K2_SetRelativeLocation` (`self.Play Button`) (`self.Play Relative Location`) false false)
  ;[1 1 1] Resets to Default when Sequence Finishes
  (`SceneComponent.K2_SetRelativeLocation` (`self.Pause_Shape`) (`self.Pause Relative Location`) false false)
  (goto _label))

(event `self.Pause_Shape.OnComponentBeginOverlap`
  (params (OverlappedComponent :type "PrimitiveComponent Object Reference") (OtherActor :type "Actor Object Reference") (OtherComp :type "PrimitiveComponent Object Reference") (OtherBodyIndex :type Integer) (bFromSweep :type Boolean) (SweepResult :type "HitResult Structure (by ref)"))
  (bind (_returnvalue_x _returnvalue_y _returnvalue_z) (`KismetMathLibrary.BreakVector` (`SceneComponent.K2_GetComponentLocation` OtherComp)))
  (bind _play_button (`self.Play Button`))
  (bind _pause_shape (`self.Pause_Shape`))
  (bind _sound (`self.Sound`))
  (bind (_returnvalue_location _returnvalue_rotation _returnvalue_scale) (`KismetMathLibrary.BreakTransform` (`SceneComponent.GetRelativeTransform` (`self.Pause_Shape`))))
  (bind (_returnvalue_x_2 _returnvalue_y_2 _returnvalue_z_2) (`KismetMathLibrary.BreakVector` (`SceneComponent.K2_GetComponentLocation` (`self.Pause_Shape`))))
  ;[0 0 0] Pause Button
  ;;[1 1 1] Conditions for Functioning
  (if (`self.Active_Pause`)
    (set `self.Active_Pause` false)
    (if (> _returnvalue_z _returnvalue_z_2)
      (if (`KismetStringLibrary.EqualEqual_StrStr` (`KismetSystemLibrary.GetObjectName` OtherComp) "HandHit")
        (if (not (`self.Is Pressed Down_Pause`))
          ;;[1 1 1] Moves Button Top
          (bind _output_get (set `self.Up Location` _returnvalue_location))
          (set `self.Return Value Rotation` _returnvalue_rotation)
          (set `self.Return Value Scale` _returnvalue_scale)
          (`SceneComponent.K2_SetRelativeTransform` (`self.Pause_Shape`) (`KismetMathLibrary.MakeTransform` (- _output_get (0.0 0.0 0.5)) (`self.Return Value Rotation`) (`self.Return Value Scale`)) false false)
          ;;[1 1 1] Playing Audio
          (`AudioComponent.SetPitchMultiplier` _sound 0.9)
          (`AudioComponent.Play` _sound 0.0)
          (set `self.Is Pressed Down_Pause` true)
          ;;[1 1 1] Released
          (`KismetSystemLibrary.Delay` 0.2)
          (if (`self.Is Pressed Down_Pause`)
            (`SceneComponent.K2_SetRelativeTransform` (`self.Pause_Shape`) (`KismetMathLibrary.MakeTransform` (`self.Up Location`) (`self.Return Value Rotation`) (`self.Return Value Scale`)) false false)
            (set `self.Is Pressed Down_Pause` false)
            ;[1 1 1] Pausing Playback
            (`AudioComponent.SetPaused` (`self.Playback`) true)
            (bind _outactors (`GameplayStatics.GetAllActorsOfClass` "/Game/Starter_Content/VirtualRealityBP/Blueprints/BP_MotionController.BP_MotionController_C"))
            (for (_ _array_index) _outactors
              (bind _asbp_motion_controller (cast `/Game/Starter_Content/VirtualRealityBP/Blueprints/BP_MotionController` (`|GetArrayItem` _outactors _array_index)))
              (set `/Game/Starter_Content/VirtualRealityBP/Blueprints/BP_MotionController.Retracking` false _asbp_motion_controller))
            (`KismetSystemLibrary.Delay` 0.2)
            (`SceneComponent.SetVisibility` (`self.Pause_Shape`) false false)
            (`SceneComponent.K2_SetRelativeLocation` _pause_shape (- (`SceneComponent.RelativeLocation` _pause_shape) (0.0 0.0 5.0)) false false)
            (`SceneComponent.SetVisibility` (`self.Play Button`) true false)
            (`SceneComponent.K2_SetRelativeLocation` _play_button (- (`SceneComponent.RelativeLocation` _play_button) (0.0 0.0 -5.0)) false false)
            (`KismetSystemLibrary.Delay` 0.8)
            (set `self.Active_Play` true))
          (else
            (`KismetSystemLibrary.PrintString` "Pressed Down Failing" true true (struct :`G` 0.66 :`B` 1.0 :`A` 1.0) 7.5)))))
    (else
      (`KismetSystemLibrary.PrintString` "Pause Active Failing" true true (struct :`R` 1.0 :`G` 0.032634 :`A` 1.0) 7.5))))

(event `self.Play Button.OnComponentBeginOverlap`
  (params (OverlappedComponent :type "PrimitiveComponent Object Reference") (OtherActor :type "Actor Object Reference") (OtherComp :type "PrimitiveComponent Object Reference") (OtherBodyIndex :type Integer) (bFromSweep :type Boolean) (SweepResult :type "HitResult Structure (by ref)"))
  (bind (_returnvalue_x _returnvalue_y _returnvalue_z) (`KismetMathLibrary.BreakVector` (`SceneComponent.K2_GetComponentLocation` OtherComp)))
  (bind _sound (`self.Sound`))
  (bind _pause_shape (`self.Pause_Shape`))
  (bind _play_button (`self.Play Button`))
  (bind _playback (`self.Playback`))
  (bind (_returnvalue_x_2 _returnvalue_y_2 _returnvalue_z_2) (`KismetMathLibrary.BreakVector` (`SceneComponent.K2_GetComponentLocation` (`self.Play Button`))))
  (bind (_returnvalue_location _returnvalue_rotation _returnvalue_scale) (`KismetMathLibrary.BreakTransform` (`SceneComponent.GetRelativeTransform` (`self.Play Button`))))
  ;[0 0 0] Play Button
  ;;[1 1 1] Conditions for Functioning
  (if (`self.Active_Play`)
    (set `self.Active_Play` false)
    (if (> _returnvalue_z _returnvalue_z_2)
      (if (`KismetStringLibrary.EqualEqual_StrStr` (`KismetSystemLibrary.GetObjectName` OtherComp) "HandHit")
        (if (not (`self.Is Pressed Down_Play`))
          ;;[1 1 1] Moves Button Top
          (bind _output_get (set `self.Up Location` _returnvalue_location))
          (set `self.Return Value Rotation` _returnvalue_rotation)
          (set `self.Return Value Scale` _returnvalue_scale)
          (`SceneComponent.K2_SetRelativeTransform` (`self.Play Button`) (`KismetMathLibrary.MakeTransform` (- _output_get (0.0 0.0 0.5)) (`self.Return Value Rotation`) (`self.Return Value Scale`)) false false)
          ;;[1 1 1] Playing Audio
          (`AudioComponent.SetPitchMultiplier` _sound 0.9)
          (`AudioComponent.Play` _sound 0.0)
          (set `self.Is Pressed Down_Play` true)
          ;;[1 1 1] Released
          (`KismetSystemLibrary.Delay` 0.2)
          (if (`self.Is Pressed Down_Play`)
            (`SceneComponent.K2_SetRelativeTransform` (`self.Play Button`) (`KismetMathLibrary.MakeTransform` (`self.Up Location`) (`self.Return Value Rotation`) (`self.Return Value Scale`)) false false)
            (set `self.Is Pressed Down_Play` false)
            (`KismetSystemLibrary.Delay` 0.25)
            (if (`self.First Time Start`)
              ;[1 1 1] First press per retrack
              (set `self.First Time Start` false)
              (set `self.Complete Flag` true)
              (bind _outactors (`GameplayStatics.GetAllActorsOfClass` "/Game/Stutter_Speak_Content/Managers/Speech_Recording.Speech_Recording_C"))
              (bind _asspeech_recording (cast `/Game/Stutter_Speak_Content/Managers/Speech_Recording` (`|GetArrayItem` _outactors)))
              (set `self.Speech Sound` (`/Game/Stutter_Speak_Content/Managers/Speech_Recording.Recorded Speech` _asspeech_recording))
              (bind _outactors_2 (`GameplayStatics.GetAllActorsOfClass` "/Game/Starter_Content/VirtualRealityBP/Blueprints/BP_MotionController.BP_MotionController_C"))
              (for (_ _array_index) _outactors_2
                (bind _asbp_motion_controller (cast `/Game/Starter_Content/VirtualRealityBP/Blueprints/BP_MotionController` (`|GetArrayItem` _outactors_2 _array_index)))
                (set `/Game/Starter_Content/VirtualRealityBP/Blueprints/BP_MotionController.Retracking` true _asbp_motion_controller))
              (`AudioComponent.Stop` (`self.Sound`))
              (`AudioComponent.SetSound` _playback (`self.Speech Sound`))
              (`AudioComponent.Play` _playback 0.0)
              (`AudioComponent.SetPaused` _playback false)
              (else
                ;[1 1 1] Subsequent pressing play
                (bind _outactors_3 (`GameplayStatics.GetAllActorsOfClass` "/Game/Starter_Content/VirtualRealityBP/Blueprints/BP_MotionController.BP_MotionController_C"))
                (for (_ _array_index_2) _outactors_3
                  (bind _asbp_motion_controller_2 (cast `/Game/Starter_Content/VirtualRealityBP/Blueprints/BP_MotionController` (`|GetArrayItem` _outactors_3 _array_index_2)))
                  (set `/Game/Starter_Content/VirtualRealityBP/Blueprints/BP_MotionController.Retracking` true _asbp_motion_controller_2))
                (`AudioComponent.SetPaused` (`self.Playback`) false)))
            (`SceneComponent.SetVisibility` (`self.Play Button`) false false)
            (`SceneComponent.K2_SetRelativeLocation` _play_button (- (`SceneComponent.RelativeLocation` _play_button) (0.0 0.0 5.0)) false false)
            (`SceneComponent.SetVisibility` (`self.Pause_Shape`) true false)
            (`SceneComponent.K2_SetRelativeLocation` _pause_shape (- (`SceneComponent.RelativeLocation` _pause_shape) (0.0 0.0 -5.0)) false false)
            (`KismetSystemLibrary.Delay` 0.8)
            (set `self.Active_Pause` true))
          (else
            (`KismetSystemLibrary.PrintString` "Pressed Down Failing" true true (struct :`G` 0.66 :`B` 1.0 :`A` 1.0) 7.5)))))
    (else
      (`KismetSystemLibrary.PrintString` "Play Active Failing" true true (struct :`G` 0.66 :`B` 1.0 :`A` 1.0) 7.5))))

(event `self.Playback.OnAudioFinished`
  (bind _play_button (`self.Play Button`))
  ;[1 1 1] Once Audio is Finished Playing
  (if (`self.Complete Flag`)
    (set `self.Complete Flag` false)
    (set `self.Active_Play` false)
    (set `self.Active_Pause` false)
    (bind _outactors (`GameplayStatics.GetAllActorsOfClass` "/Game/Starter_Content/VirtualRealityBP/Blueprints/BP_MotionController.BP_MotionController_C"))
    (for (_ _array_index) _outactors
      (bind _asbp_motion_controller (cast `/Game/Starter_Content/VirtualRealityBP/Blueprints/BP_MotionController` (`|GetArrayItem` _outactors _array_index)))
      (set `/Game/Starter_Content/VirtualRealityBP/Blueprints/BP_MotionController.Retracking` false _asbp_motion_controller)
      (bind _outactors_2 (`GameplayStatics.GetAllActorsOfClass` "/Game/Stutter_Speak_Content/Managers/Stutter_Timer__Empty_Object__Blueprint.Stutter_Timer__Empty_Object__Blueprint_C"))
      (bind _asstutter_timer__empty_object__blueprint (cast `/Game/Stutter_Speak_Content/Managers/Stutter_Timer__Empty_Object__Blueprint` (`|GetArrayItem` _outactors_2)))
      (`/Game/Stutter_Speak_Content/Managers/Stutter_Timer__Empty_Object__Blueprint.Stop Timer` _asstutter_timer__empty_object__blueprint)
      (`/Game/Stutter_Speak_Content/Managers/Stutter_Timer__Empty_Object__Blueprint.Clear Timer` _asstutter_timer__empty_object__blueprint)
      (if (`self.FirstTime`)
        (set `self.FirstTime` false)
        (bind _asmenu_gi (cast `/Game/Stutter_Speak_Content/Blueprints/MenuGI` (`GameplayStatics.GetGameInstance`)))
        (set `self.Inital Total Time Stuttering` (`/Game/Stutter_Speak_Content/Blueprints/MenuGI.Data to Save : Total Time Stuttering` _asmenu_gi)))
      (`/Game/Stutter_Speak_Content/Blueprints/MenuGI.SaveOverTotalTimeStuttering` _asmenu_gi)
      (bind _outactors_3 (`GameplayStatics.GetAllActorsOfClass` "/Game/Stutter_Speak_Content/Blueprints/Hanging_Projector_Screen_Blueprint.Hanging_Projector_Screen_Blueprint_C"))
      (bind _ashanging_projector_screen_blueprint (cast `/Game/Stutter_Speak_Content/Blueprints/Hanging_Projector_Screen_Blueprint` (`|GetArrayItem` _outactors_3)))
      (`/Game/Stutter_Speak_Content/Widgets/Speech_World/ResultsDataBP.ResultsCallbyConfirmRatingButton` (`/Game/Stutter_Speak_Content/Blueprints/Hanging_Projector_Screen_Blueprint.Results Data` _ashanging_projector_screen_blueprint))
      (`/Game/Stutter_Speak_Content/Widgets/Speech_World/Retracking_Results.UpdateDataByPausePlayButton` (`/Game/Stutter_Speak_Content/Blueprints/Hanging_Projector_Screen_Blueprint.Retracking Results` _ashanging_projector_screen_blueprint) (`self.Inital Total Time Stuttering`))
      (`/Game/Stutter_Speak_Content/Blueprints/Hanging_Projector_Screen_Blueprint.DisplayRetrackingResults` _ashanging_projector_screen_blueprint)
      (`PrimitiveComponent.SetMaterial` (`self.Play Button`) 0 "/Game/Stutter_Speak_Content/Materials/MenuWorldMiscMaterials/SettingsBox.SettingsBox" :!label _label_2)
      (`PrimitiveComponent.SetMaterial` (`self.Pause_Shape`) 0 "/Game/Stutter_Speak_Content/Materials/MenuWorldMiscMaterials/SettingsBox.SettingsBox")
      (`PrimitiveComponent.SetMaterial` (`self.Pause_Shape`) 1 "/Game/Stutter_Speak_Content/Materials/MenuWorldMiscMaterials/SettingsBox.SettingsBox")
      (`SceneComponent.SetVisibility` (`self.Play Button`) true false)
      (`SceneComponent.SetVisibility` (`self.Pause_Shape`) false false)
      (`SceneComponent.K2_SetRelativeLocation` _play_button (- (`SceneComponent.RelativeLocation` _play_button) (0.0 0.0 -2.5)) false false))))

(event `RaiseButton`
  (bind _defaultsceneroot (`self.DefaultSceneRoot`))
  (bind _pause_shape (`self.Pause_Shape`))
  ;[1 1 1] Raises Button When Called
  (`self.SetActorHiddenInGame` false)
  (`KismetSystemLibrary.MoveComponentTo` _defaultsceneroot (+ (`SceneComponent.RelativeLocation` _defaultsceneroot) (0.0 0.0 7.5)) (`SceneComponent.RelativeRotation` _defaultsceneroot) false false 1.0)
  (set `self.Play Relative Location` (`SceneComponent.RelativeLocation` (`self.Play Button`)))
  (set `self.Pause Relative Location` (`SceneComponent.RelativeLocation` (`self.Pause_Shape`)))
  (`SceneComponent.K2_SetRelativeLocation` _pause_shape (- (`SceneComponent.RelativeLocation` _pause_shape) (0.0 0.0 5.0)) false false)
  (`KismetSystemLibrary.Delay` 0.4)
  (set `self.Active_Play` true))

(event `ForceStop`
  (bind _playback (`self.Playback`))
  ;[1 1 1] Stops Media Prematurely if needed
  (`/Engine/EditorBlueprintResources/StandardMacros.IsValid` _playback
    (:`Is Valid`
      (`AudioComponent.SetPaused` _playback true)
      (set `self.Active_Play` false)
      (set `self.Active_Pause` false)
      (goto _label_2))))

(event `Lower Button`
  (bind _defaultsceneroot (`self.DefaultSceneRoot`))
  ;[1 1 1] Lower Button when Called
  (set `self.Active_Pause` false)
  (set `self.Active_Play` false)
  (`KismetSystemLibrary.MoveComponentTo` _defaultsceneroot (+ (`SceneComponent.RelativeLocation` _defaultsceneroot) (0.0 0.0 -7.5)) (`SceneComponent.RelativeRotation` _defaultsceneroot) false false 1.0)
  (`self.SetActorHiddenInGame` true)
  (`self.Reset`))

(fn `UserConstructionScript`)