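; SliderBP is a hand-operated on/off settings switch, with the actor's first tag selecting which audio, microphone or stutter-tracker option it controls.
; After a one-second delay on BeginPlay, it reads MenuGI to set slider position, LED material and name label.
; Overlap by a HandHit component calls the matching SettingsBox toggle, plays a sound and flips slider and LED, with a half-second Grabbable debounce.
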(event `self.ReceiveBeginPlay`
  (bind _slider (`self.Slider`))
  (bind _led (`self.LED`))
  (bind _output (`|GetArrayItem` (`self.Tags`)))
  (bind _returnvalue (`KismetStringLibrary.ParseIntoArray` (`KismetStringLibrary.Conv_NameToString` _output)))
  ;[1 1 1] Sets correct positioning and grabbability on spawn
  (`KismetSystemLibrary.Delay` 1.0)
  (bind _asmenu_gi (cast `/Game/Stutter_Speak_Content/Blueprints/MenuGI` (`GameplayStatics.GetGameInstance`)))
  (switch `string` (`KismetStringLibrary.Conv_NameToString` (`|GetArrayItem` (`self.Tags`)))
    (:`Microphone Indicator`
      (if (`/Game/Stutter_Speak_Content/Blueprints/MenuGI.MicrophoneColor` _asmenu_gi)
        (`SceneComponent.K2_SetRelativeLocation` _slider (0.0 24.0 0.0) false false :!label _label)
        (`PrimitiveComponent.SetMaterial` _led 0 "/Game/Stutter_Speak_Content/Materials/MenuWorldMiscMaterials/LED_On.LED_On")
        (else
          (`SceneComponent.K2_SetRelativeLocation` _slider (0.0 -24.0 0.0) false false :!label _label_2)
          (`PrimitiveComponent.SetMaterial` _led 0 "/Game/Stutter_Speak_Content/Materials/MenuWorldMiscMaterials/LED_Off.LED_Off")
          (`KismetSystemLibrary.PrintString` "off" true true (struct :`G` 0.66 :`B` 1.0 :`A` 1.0) 20.0))))
    (:`Physical Stutter Tracker`
      (if (`/Game/Stutter_Speak_Content/Blueprints/MenuGI.StutterButtonOn` _asmenu_gi)
        (goto _label)
        (else
          (goto _label_2))))
    (:`Audience Applause`
      (if (`/Game/Stutter_Speak_Content/Blueprints/MenuGI.Applause` _asmenu_gi)
        (goto _label)
        (else
          (goto _label_2))))
    (:`Ambient Audience Sounds`
      (if (`/Game/Stutter_Speak_Content/Blueprints/MenuGI.Ambience` _asmenu_gi)
        (goto _label)
        (else
          (goto _label_2))))
    (:`Menu Music`
      (if (`/Game/Stutter_Speak_Content/Blueprints/MenuGI.MenuMusic` _asmenu_gi)
        (goto _label)
        (else
          (goto _label_2)))))
  (if (> (`KismetArrayLibrary.Array_Length` _returnvalue) 2)
    (set `self.SettingName` (`KismetTextLibrary.Conv_StringToText` (`KismetStringLibrary.Concat_StrStr` (`|GetArrayItem` _returnvalue) " " (`|GetArrayItem` _returnvalue 1) " \n" (`|GetArrayItem` _returnvalue 2))))
    (else
      (set `self.SettingName` (`KismetTextLibrary.Conv_NameToText` _output))))
  (`TextRenderComponent.K2_SetText` (`self.Name`) (`self.SettingName`)))

(event `/Game/Starter_Content/VirtualRealityBP/Blueprints/PickupActorInterface.Pickup`
  (params (AttachTo :type "SceneComponent Object Reference")))

(event `self.Slider.OnComponentBeginOverlap`
  (params (OverlappedComponent :type "PrimitiveComponent Object Reference") (OtherActor :type "Actor Object Reference") (OtherComp :type "PrimitiveComponent Object Reference") (OtherBodyIndex :type Integer) (bFromSweep :type Boolean) (SweepResult :type "HitResult Structure (by ref)"))
  (bind _led (`self.LED`))
  (bind _slider (`self.Slider`))
  (bind (_relativelocation_x _relativelocation_y) (`KismetMathLibrary.BreakVector` (`SceneComponent.RelativeLocation` (`self.Slider`))))
  ;[1 1 1] On grab, updates position and save data
  (if (`KismetStringLibrary.EqualEqual_StrStr` (`KismetSystemLibrary.GetObjectName` OtherComp) "HandHit")
    (if (`self.Grabbable`)
      (set `self.Grabbable` false)
      (bind _returnvalue (`GameplayStatics.GetActorOfClass` "/Game/Stutter_Speak_Content/Blueprints/SettingsBox.SettingsBox_C"))
      (bind _assettings_box (cast `/Game/Stutter_Speak_Content/Blueprints/SettingsBox` _returnvalue))
      (bind _output_get (set `self.As Settings Box` _assettings_box))
      (switch `string` (`KismetStringLibrary.Conv_NameToString` (`|GetArrayItem` (`self.Tags`)))
        (:`Microphone Indicator`
          (`/Game/Stutter_Speak_Content/Blueprints/SettingsBox.MicrophoneColorByMicSwitch` _output_get))
        (:`Physical Stutter Tracker`
          (`/Game/Stutter_Speak_Content/Blueprints/SettingsBox.StutterButtonByStutterSwitch` _output_get))
        (:`Audience Applause`
          (`/Game/Stutter_Speak_Content/Blueprints/SettingsBox.ApplauseByApplauseSwitch` _output_get))
        (:`Ambient Audience Sounds`
          (`/Game/Stutter_Speak_Content/Blueprints/SettingsBox.AmbienceByAmbienceSwitch` _output_get))
        (:`Menu Music`
          (`/Game/Stutter_Speak_Content/Blueprints/SettingsBox.MusicOnByMusicSwitch` _output_get)))
      (`AudioComponent.Play` (`self.Sound On`) 0.0)
      (if (< _relativelocation_y 0.0)
        (`SceneComponent.K2_SetRelativeLocation` _slider (0.0 24.0 0.0) false false)
        (`PrimitiveComponent.SetMaterial` _led 0 "/Game/Stutter_Speak_Content/Materials/MenuWorldMiscMaterials/LED_On.LED_On")
        (else
          (`SceneComponent.K2_SetRelativeLocation` _slider (0.0 -24.0 0.0) false false)
          (`PrimitiveComponent.SetMaterial` _led 0 "/Game/Stutter_Speak_Content/Materials/MenuWorldMiscMaterials/LED_Off.LED_Off")))
      (`KismetSystemLibrary.Delay` 0.5)
      (set `self.Grabbable` true))))

(fn `UserConstructionScript`)