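; Trigger box Blueprint that toggles a VR hand's pointer and widget interaction as that motion controller enters or leaves overlap.
; Externally called unhide and hide events match the overlapper to the left or right hand, then show or hide its pointer and activate or deactivate its WidgetInteraction.
; Active flags let only one hand hold the pointer at a time.
; The delayed GetAllActorsOfClass lookup that fills hand and pointer references is disconnected and never runs.
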(event `LeftHandUnhideByExternal`
  (params (Overlapper :type "Actor Object Reference"))
  (bind _left_pointer (`self.Left Pointer`))
  ;[1 1 1] Unhides Specific Pointer When Overlaps with Trigger Box and Disables Widget Interaction
  (if (and (== false (`self.Right Hand Active`)) (== Overlapper (`self.Left Hand`)))
    (set `self.Left Hand Active` true)
    (`ActorComponent.Activate` (`/Game/Starter_Content/VirtualRealityBP/Blueprints/BP_MotionController.WidgetInteraction` (`self.Left Hand`)) false)
    (`SceneComponent.SetHiddenInGame` _left_pointer false false)
    (`SceneComponent.SetVisibility` _left_pointer true false)))

(event `RightHandUnhideByExternal`
  (params (Overlapper :type "Actor Object Reference"))
  (bind _right_pointer (`self.Right Pointer`))
  ;[1 1 1] Unhides Specific Pointer When Overlaps with Trigger Box and Disables Widget Interaction
  (if (and (== Overlapper (`self.Right Hand`)) (== (`self.Left Hand Active`) false))
    (set `self.Right Hand Active` true)
    (`ActorComponent.Activate` (`/Game/Starter_Content/VirtualRealityBP/Blueprints/BP_MotionController.WidgetInteraction` (`self.Right Hand`)) false)
    (`SceneComponent.SetHiddenInGame` _right_pointer false false)
    (`SceneComponent.SetVisibility` _right_pointer true false)))

(event `LeftHandHiddenByExternal`
  (params (Overlapper :type "Actor Object Reference"))
  (bind _left_pointer (`self.Left Pointer`))
  ;[1 1 1] Hides Specific Pointer When Leaves Overlap of Trigger Box and Disables Widget Interaction
  (if (and (== false (`self.Right Hand Active`)) (== Overlapper (`self.Left Hand`)))
    (set `self.Left Hand Active` false)
    (`SceneComponent.SetHiddenInGame` _left_pointer true false)
    (`SceneComponent.SetVisibility` _left_pointer true false)
    (`ActorComponent.Deactivate` (`/Game/Starter_Content/VirtualRealityBP/Blueprints/BP_MotionController.WidgetInteraction` (`self.Left Hand`)))))

(event `RightHandHiddenByExternal`
  (params (Overlapper :type "Actor Object Reference"))
  (bind _right_pointer (`self.Right Pointer`))
  ;[1 1 1] Hides Specific Pointer When Leaves Overlap of Trigger Box and Disables Widget Interaction
  (if (and (== Overlapper (`self.Right Hand`)) (== (`self.Left Hand Active`) false))
    (set `self.Right Hand Active` false)
    (`SceneComponent.SetHiddenInGame` _right_pointer true false)
    (`SceneComponent.SetVisibility` _right_pointer true false)
    (`ActorComponent.Deactivate` (`/Game/Starter_Content/VirtualRealityBP/Blueprints/BP_MotionController.WidgetInteraction` (`self.Right Hand`)))))

(fn `UserConstructionScript`)