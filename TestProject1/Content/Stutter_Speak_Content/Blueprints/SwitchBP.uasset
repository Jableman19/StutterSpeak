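; Grabbable toggle switch for the settings box, with its first actor tag selecting the option it controls: microphone color, stutter button, applause, music or one of three text sizes.
; On BeginPlay it reads MenuGI to set the switch's tilt and locks the active text-size switch.
; On pickup it calls the matching SettingsBox function and flips the tilt.
; Text-size switches then disable their own grabbing, so the selected size cannot be toggled off directly.
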(event `self.ReceiveBeginPlay`
  (bind _switch (`self.Switch`))
  ;[1 1 1] Sets correct positioning and grabbability on spawn
  (bind _asmenu_gi (cast `/Game/Stutter_Speak_Content/Blueprints/MenuGI` (`GameplayStatics.GetGameInstance`)))
  (switch `string` (`KismetStringLibrary.Conv_NameToString` (`|GetArrayItem` (`self.Tags`)))
    (:`Microphone`
      (if (`/Game/Stutter_Speak_Content/Blueprints/MenuGI.MicrophoneColor` _asmenu_gi)
        (`SceneComponent.K2_SetRelativeRotation` _switch (struct :`Roll` -30.0) false false :!label _label)
        (else
          (`SceneComponent.K2_SetRelativeRotation` _switch (struct :`Roll` 30.0) false false :!label _label_2))))
    (:`Stutter`
      (if (`/Game/Stutter_Speak_Content/Blueprints/MenuGI.StutterButtonOn` _asmenu_gi)
        (goto _label)
        (else
          (goto _label_2))))
    (:`Applause`
      (if (`/Game/Stutter_Speak_Content/Blueprints/MenuGI.Applause` _asmenu_gi)
        (goto _label)
        (else
          (goto _label_2))))
    (:`Music`
      (if (`/Game/Stutter_Speak_Content/Blueprints/MenuGI.MenuMusic` _asmenu_gi)
        (goto _label)
        (else
          (goto _label_2))))
    (:`Large`
      (bind _textsize (`/Game/Stutter_Speak_Content/Blueprints/MenuGI.TextSize` _asmenu_gi))
      (if (`KismetStringLibrary.EqualEqual_StrStr` _textsize "Large")
        (set `self.Grabbable` false)
        (goto _label)
        (else
          (goto _label_2))))
    (:`Medium`
      (if (`KismetStringLibrary.EqualEqual_StrStr` _textsize "Medium")
        (set `self.Grabbable` false)
        (goto _label)
        (else
          (goto _label_2))))
    (:`Small`
      (if (`KismetStringLibrary.EqualEqual_StrStr` _textsize "Small")
        (set `self.Grabbable` false)
        (goto _label)
        (else
          (goto _label_2))))))

(event `/Game/Starter_Content/VirtualRealityBP/Blueprints/PickupActorInterface.Pickup`
  (params (AttachTo :type "SceneComponent Object Reference"))
  (bind _switch (`self.Switch`))
  (bind _relativerotation_roll (`KismetMathLibrary.BreakRotator` (`SceneComponent.RelativeRotation` (`self.Switch`))))
  ;[1 1 1] On grab, updates position and save data
  (if (`self.Grabbable`)
    (bind _returnvalue (`GameplayStatics.GetActorOfClass` "/Game/Stutter_Speak_Content/Blueprints/SettingsBox.SettingsBox_C"))
    (bind _assettings_box (cast `/Game/Stutter_Speak_Content/Blueprints/SettingsBox` _returnvalue))
    (bind _output_get (set `self.As Settings Box` _assettings_box))
    (switch `string` (`KismetStringLibrary.Conv_NameToString` (`|GetArrayItem` (`self.Tags`)))
      (:`Microphone`
        (`/Game/Stutter_Speak_Content/Blueprints/SettingsBox.MicrophoneColorByMicSwitch` _output_get))
      (:`Stutter`
        (`/Game/Stutter_Speak_Content/Blueprints/SettingsBox.StutterButtonByStutterSwitch` _output_get))
      (:`Applause`
        (`/Game/Stutter_Speak_Content/Blueprints/SettingsBox.ApplauseByApplauseSwitch` _output_get))
      (:`Music`
        (`/Game/Stutter_Speak_Content/Blueprints/SettingsBox.MusicOnByMusicSwitch` _output_get))
      (:`Large`
        (`/Game/Stutter_Speak_Content/Blueprints/SettingsBox.LargeByLargeSwitch` _output_get)
        (set `self.Grabbable` false :!label _label_3))
      (:`Medium`
        (`/Game/Stutter_Speak_Content/Blueprints/SettingsBox.MediumByMediumSwitch` _output_get)
        (goto _label_3))
      (:`Small`
        (`/Game/Stutter_Speak_Content/Blueprints/SettingsBox.SmallBySmallSwitch` _output_get)
        (goto _label_3)))
    (if (< _relativerotation_roll 0.0)
      (`SceneComponent.K2_SetRelativeRotation` _switch (struct :`Roll` 30.0) false false)
      (else
        (`SceneComponent.K2_SetRelativeRotation` _switch (struct :`Roll` -30.0) false false)))))

(fn `UserConstructionScript`)